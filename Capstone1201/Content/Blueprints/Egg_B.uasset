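; Egg_B is a possessable Knight egg unit that fights Egg_W units by collision.
; While possessed it supports camera turn and zoom; clicking it starts aiming, rotating the egg away from the cursor and stretching an arrow by distance.
; Hitting an Egg_W after a click cuts its health, plays combat animations and spawns Crash_Actor text.
; Fire-zone overlaps only set a burning flag; fire damage and death are functions not called here.
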(event `self.ReceiveUnpossessed`
  (params (OldController :type "Controller Object Reference"))
  (bind _springarm (`self.SpringArm`))
  ;[1 1 1] 조준 도중, 혹은 포커스 된 상태에서 우클릭 시 화살, possessed 변수처리
  (set `self.B_possessed` false)
  (`SceneComponent.SetVisibility` (`self.Arrow`) false false)
  (`SkeletalMeshComponent.PlayAnimation` (`self.Knight`) "/Game/Charactor/Animations/Basic_idle.Basic_idle" true)
  (set `SpringArmComponent.TargetArmLength` 1000.0 _springarm)
  (`SceneComponent.K2_SetRelativeRotation` _springarm (struct :`Pitch` -50.0) false false))

(event `self.ReceivePossessed`
  (params (NewController :type "Controller Object Reference"))
  ;[1 1 1] 조준 도중, 혹은 포커스 된 상태에서 우클릭 시 화살, possessed 변수처리
  (`SkeletalMeshComponent.PlayAnimation` (`self.Knight`) "/Game/Charactor/Animations/Selected.Selected" true))

(event `self.ReceiveTick`
  (params (DeltaSeconds :type "Float (single-precision)"))
  ;[1 1 1] 액터 클릭에 대한 처리, 화살 표시, 플레이어가 선택한 캐릭터 표시 처리
  (if (`self.B_possessed`)
    (`SceneComponent.SetVisibility` (`self.Active`) true false)
    (if (`self.Egg Clicked_B`)
      (`self.Rotate Arrow` (stale `self.Egg.OnClicked` _egg_position)))
    (else
      (`SceneComponent.SetVisibility` (`self.Active`) false false))))

(event `self.Egg.OnClicked`
  (params (TouchedComponent :type "PrimitiveComponent Object Reference") (ButtonPressed :type "Key Structure"))
  ;[1 1 1] 액터 클릭에 대한 처리, 화살 표시, 플레이어가 선택한 캐릭터 표시 처리
  (if (`self.B_possessed`)
    (bind _egg_position (`self.Egg_Click`))))

(event `self.ReceiveHit`
  (params (MyComp :type "PrimitiveComponent Object Reference") (Other :type "Actor Object Reference") (OtherComp :type "PrimitiveComponent Object Reference") (bSelfMoved :type Boolean) (HitLocation :type "Vector Structure") (HitNormal :type "Vector Structure") (NormalImpulse :type "Vector Structure") (Hit :type "HitResult Structure (by ref)"))
  (bind _returnvalue (`SceneComponent.K2_GetComponentLocation` (`self.Egg`)))
  ;[1 1 1] 충돌 시 텍스트 출력(텍스트는 블루프린트로 되어 있음 = 블루프린트 폴더의 Crash_Actor)
  (if (`self.Egg Clicked_B`)
    (bind _asegg_w (cast `/Game/Blueprints/Egg_W` Other))
    (`self.Reduce_Health` _asegg_w)
    (`SkeletalMeshComponent.PlayAnimation` (`/Game/Blueprints/Egg_W.Knight` _asegg_w) "/Game/Charactor/Animations/Attacked.Attacked" true)
    (`SkeletalMeshComponent.PlayAnimation` (`self.Knight`) "/Game/Charactor/Animations/Slash.Slash" true)
    (set `self.IsCrashed_B` true)
    (set `self.CrashPos_B` (+ _returnvalue (0.0 0.0 1500.0)))
    (`|SpawnActorFromClass` "/Game/Blueprints/Crash_Actor.Crash_Actor_C" (`KismetMathLibrary.Conv_VectorToTransform` (+ _returnvalue (0.0 0.0 10.0))) "Undefined" "OverrideRootScale" null null)))

(event `InputAxis|Turn`
  (params (AxisValue :type "Float (single-precision)"))
  ;[1 1 1] 알 빙의 후, A,D키를 눌러 화면을 돌려가며 볼 수 있게 함
  (if (`self.B_possessed`)
    (`SceneComponent.K2_AddWorldRotation` (`self.SpringArm`) (`KismetMathLibrary.MakeRotator` 0.0 0.0 AxisValue) false true)))

(event `InputAxis|Zoom`
  (params (AxisValue :type "Float (single-precision)"))
  (bind _springarm (`self.SpringArm`))
  ;[1 1 1] 알 빙의 후, 휠을 이용해 화면 확대, 축소 가능
  (if (`self.B_possessed`)
    (set `SpringArmComponent.TargetArmLength` (+ (* AxisValue 100.0) (`SpringArmComponent.TargetArmLength` _springarm)) _springarm)))

(event `self.ReceiveActorBeginOverlap`
  (params (OtherActor :type "Actor Object Reference"))
  (bind _returnvalue (`GameplayStatics.GetObjectClass` OtherActor))
  ;[1 1 1] 불장판에 닿으면 health 20 감소, isOnFire를 True로 변경
  (if (or (== _returnvalue "/Game/Blueprints/BP_Fire_Zone_75per.BP_Fire_Zone_75per_C") (== _returnvalue "/Game/Blueprints/BP_Fire_Zone_60per.BP_Fire_Zone_60per_C") (== _returnvalue "/Game/Blueprints/BP_Fire_Zone_50per.BP_Fire_Zone_50per_C") (== _returnvalue "/Game/Blueprints/BP_Fire_Zone_40per.BP_Fire_Zone_40per_C"))
    (set `self.isOnFire(B)` true)))

(event `self.ReceiveActorEndOverlap`
  (params (OtherActor :type "Actor Object Reference"))
  (bind _returnvalue (`GameplayStatics.GetObjectClass` OtherActor))
  ;[1 1 1] 불에서 빠져나오면 isOnFire를 False로 변경
  (if (or (== _returnvalue "/Game/Blueprints/BP_Fire_Zone_75per.BP_Fire_Zone_75per_C") (== _returnvalue "/Game/Blueprints/BP_Fire_Zone_60per.BP_Fire_Zone_60per_C") (== _returnvalue "/Game/Blueprints/BP_Fire_Zone_50per.BP_Fire_Zone_50per_C") (== _returnvalue "/Game/Blueprints/BP_Fire_Zone_40per.BP_Fire_Zone_40per_C"))
    (set `self.isOnFire(B)` false)))

(fn `Egg_Click`
  (returns (`Egg Position` :type "Vector Structure"))
  (set `self.Egg Clicked_B` true)
  (bind _output_get (set `self.Egg_Pos_B` (`SceneComponent.K2_GetComponentLocation` (`self.Egg`))))
  (`KismetSystemLibrary.PrintText` (`KismetTextLibrary.Conv_VectorToText` _output_get))
  (return _output_get))

(fn `Reduce_Health`
  (params (`damaged egg` :type "/Game/Blueprints/Egg_W Object Reference"))
  (bind _output_get (set `/Game/Blueprints/Egg_W.health(W)` (- (`/Game/Blueprints/Egg_W.health(W)` `damaged egg`) 20.0) `damaged egg`))
  (set `/Game/Blueprints/Egg_W.hp_percent(W)` (/ _output_get 100.0) `damaged egg`))

(fn `Rotate Arrow`
  (params (`Egg Position` :type "Vector Structure"))
  (bind (_bblockinghit _binitialoverlap _time _distance _location _impactpoint _normal _impactnormal _physmat _hitactor) (`GameplayStatics.BreakHitResult` (`PlayerController.GetHitResultUnderCursorByChannel` (`GameplayStatics.GetPlayerController` 0) "TraceTypeQuery1" true)))
  (`SceneComponent.SetVisibility` (`self.Arrow`) true false)
  (cast `/Game/Blueprints/Egg_B` _hitactor
    (:`CastFailed`
      (bind _output_get (set `self.Egg_Rotation` (`KismetMathLibrary.Conv_VectorToRotator` (- `Egg Position` (`KismetMathLibrary.MakeVector` (.x _location) (.y _location) (.z `Egg Position`))))))
      (`SceneComponent.K2_SetWorldRotation` (`self.Egg`) _output_get false false)
      (`SceneComponent.SetWorldScale3D` (`self.Arrow`) (`KismetMathLibrary.MakeVector` (/ (`KismetMathLibrary.Sqrt` (`KismetMathLibrary.DistanceSquared2D` (`KismetMathLibrary.Conv_VectorToVector2D` _location) (`KismetMathLibrary.Conv_VectorToVector2D` `Egg Position`))) 60.0) 5.0 5.0)))))

(fn `Set Unit Dead(B)`
  (set `self.isDead(B)` true)
  (`self.SetActorHiddenInGame` true)
  (`self.SetActorEnableCollision` false))

(fn `Take Fire Damage(B)`
  (bind _output_get (set `self.health(B)` (- (`self.health(B)`) 20.0)))
  (set `self.hp_percent(B)` (/ _output_get 100.0)))

(fn `UserConstructionScript`)