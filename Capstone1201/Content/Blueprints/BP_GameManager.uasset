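; Game manager for a turn-based White versus Black battle with five units per team, handling burn damage, deaths and victory.
; BeginPlay caches both team arrays into per-unit variables after a short delay and starts battle music.
; Each turn-start event applies fire damage to the opposing team's burning units.
; CheckUnitsSurvival kills units at zero health and shows the winner's widget when a whole team is dead.
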(event `self.ReceiveBeginPlay`
  (`KismetSystemLibrary.Delay` 0.2)
  (`self.set_white_team_from_array`)
  (`self.set_black_team_from_array`)
  (`GameplayStatics.PlaySound2D` "/Game/Sounds/battleThemeA.battleThemeA" 0.2 0.8 0.0 null null))

(event `self.ReceiveTick`
  (params (DeltaSeconds :type "Float (single-precision)")))

(event `White Turn Starts(GM)`
  (`KismetSystemLibrary.PrintString` "wite turn starts(GM)")
  (`self.Apply Fire Gamage(B)`))

(event `Black Turn Starts(GM)`
  (`KismetSystemLibrary.PrintString` "black turn starts(GM)")
  (`self.Apply Fire Damage(W)`))

(fn `Apply Fire Damage(W)`
  (`|ExecutionSequence`
    (:`then_0`
      (if (`/Game/Blueprints/Egg_W.isOnFire(W)` (`self.white1`))
        (`/Game/Blueprints/Egg_W.Take Fire Damage(W)` (`self.white1`))))
    (:`then_1`
      (if (`/Game/Blueprints/Egg_W.isOnFire(W)` (`self.white2`))
        (`/Game/Blueprints/Egg_W.Take Fire Damage(W)` (`self.white2`))))
    (:`then_2`
      (if (`/Game/Blueprints/Egg_W.isOnFire(W)` (`self.white3`))
        (`/Game/Blueprints/Egg_W.Take Fire Damage(W)` (`self.white3`))))
    (:`then_3`
      (if (`/Game/Blueprints/Egg_W.isOnFire(W)` (`self.white4`))
        (`/Game/Blueprints/Egg_W.Take Fire Damage(W)` (`self.white4`))))
    (:`then_4`
      (if (`/Game/Blueprints/Egg_W.isOnFire(W)` (`self.white5`))
        (`/Game/Blueprints/Egg_W.Take Fire Damage(W)` (`self.white5`))))))

(fn `Apply Fire Gamage(B)`
  (`|ExecutionSequence`
    (:`then_0`
      (if (`/Game/Blueprints/Egg_B.isOnFire(B)` (`self.black1`))
        (`/Game/Blueprints/Egg_B.Take Fire Damage(B)` (`self.black1`))))
    (:`then_1`
      (if (`/Game/Blueprints/Egg_B.isOnFire(B)` (`self.black2`))
        (`/Game/Blueprints/Egg_B.Take Fire Damage(B)` (`self.black2`))))
    (:`then_2`
      (if (`/Game/Blueprints/Egg_B.isOnFire(B)` (`self.black3`))
        (`/Game/Blueprints/Egg_B.Take Fire Damage(B)` (`self.black3`))))
    (:`then_3`
      (if (`/Game/Blueprints/Egg_B.isOnFire(B)` (`self.black4`))
        (`/Game/Blueprints/Egg_B.Take Fire Damage(B)` (`self.black4`))))
    (:`then_4`
      (if (`/Game/Blueprints/Egg_B.isOnFire(B)` (`self.black5`))
        (`/Game/Blueprints/Egg_B.Take Fire Damage(B)` (`self.black5`))))))

(fn `Black Wins`
  (`KismetSystemLibrary.PrintString` "흑돌 승리!")
  (`Widget.SetVisibility` (`self.level_UI(gm)`) "Hidden")
  (bind _returnvalue (`|CreateWidget` "/Game/Blueprints/BP_Black_Win.BP_Black_Win_C"))
  (`UserWidget.AddToViewport` _returnvalue 0))

(fn `Check Units Survival`
  (`|ExecutionSequence`
    (:`then_0`
      ;[1 1 1] 각 유닛의 체력을 확인하여 0이하이면 사망처리
      (if (<= (`/Game/Blueprints/Egg_W.health(W)` (`self.white1`)) 0.0)
        (`/Game/Blueprints/Egg_W.Set Unit Dead(W)` (`self.white1`))))
    (:`then_1`
      (if (<= (`/Game/Blueprints/Egg_W.health(W)` (`self.white2`)) 0.0)
        (`/Game/Blueprints/Egg_W.Set Unit Dead(W)` (`self.white2`))))
    (:`then_2`
      (if (<= (`/Game/Blueprints/Egg_W.health(W)` (`self.white3`)) 0.0)
        (`/Game/Blueprints/Egg_W.Set Unit Dead(W)` (`self.white3`))))
    (:`then_3`
      (if (<= (`/Game/Blueprints/Egg_W.health(W)` (`self.white4`)) 0.0)
        (`/Game/Blueprints/Egg_W.Set Unit Dead(W)` (`self.white4`))))
    (:`then_4`
      (if (<= (`/Game/Blueprints/Egg_W.health(W)` (`self.white5`)) 0.0)
        (`/Game/Blueprints/Egg_W.Set Unit Dead(W)` (`self.white5`))))
    (:`then_5`
      (if (<= (`/Game/Blueprints/Egg_B.health(B)` (`self.black1`)) 0.0)
        (`/Game/Blueprints/Egg_B.Set Unit Dead(B)` (`self.black1`))))
    (:`then_6`
      (if (<= (`/Game/Blueprints/Egg_B.health(B)` (`self.black2`)) 0.0)
        (`/Game/Blueprints/Egg_B.Set Unit Dead(B)` (`self.black2`))))
    (:`then_7`
      (if (<= (`/Game/Blueprints/Egg_B.health(B)` (`self.black3`)) 0.0)
        (`/Game/Blueprints/Egg_B.Set Unit Dead(B)` (`self.black3`))))
    (:`then_8`
      (if (<= (`/Game/Blueprints/Egg_B.health(B)` (`self.black4`)) 0.0)
        (`/Game/Blueprints/Egg_B.Set Unit Dead(B)` (`self.black4`))))
    (:`then_9`
      (if (<= (`/Game/Blueprints/Egg_B.health(B)` (`self.black5`)) 0.0)
        (`/Game/Blueprints/Egg_B.Set Unit Dead(B)` (`self.black5`))))
    (:`then_10`
      (`|ExecutionSequence`
        (:`then_0`
          (if (and (`/Game/Blueprints/Egg_W.isDead(W)` (`self.white1`)) (`/Game/Blueprints/Egg_W.isDead(W)` (`self.white2`)) (`/Game/Blueprints/Egg_W.isDead(W)` (`self.white3`)) (`/Game/Blueprints/Egg_W.isDead(W)` (`self.white4`)) (`/Game/Blueprints/Egg_W.isDead(W)` (`self.white5`)))
            (`self.Black Wins`)))
        (:`then_1`
          (if (and (`/Game/Blueprints/Egg_B.isDead(B)` (`self.black1`)) (`/Game/Blueprints/Egg_B.isDead(B)` (`self.black2`)) (`/Game/Blueprints/Egg_B.isDead(B)` (`self.black3`)) (`/Game/Blueprints/Egg_B.isDead(B)` (`self.black4`)) (`/Game/Blueprints/Egg_B.isDead(B)` (`self.black5`)))
            (`self.White Wins`)))))))

(fn `Set Units State Hidden`
  (bind _level_ui_gm_ (`self.level_UI(gm)`))
  (`Widget.SetVisibility` (`/Game/Blueprints/BP_Level_UI.HorizontalBox_B_Team` _level_ui_gm_) "Hidden")
  (`Widget.SetVisibility` (`/Game/Blueprints/BP_Level_UI.HorizontalBox_W_Team` _level_ui_gm_) "Hidden"))

(fn `Set Units State Visible`
  (bind _level_ui_gm_ (`self.level_UI(gm)`))
  (`Widget.SetVisibility` (`/Game/Blueprints/BP_Level_UI.HorizontalBox_B_Team` _level_ui_gm_) "SelfHitTestInvisible")
  (`Widget.SetVisibility` (`/Game/Blueprints/BP_Level_UI.HorizontalBox_W_Team` _level_ui_gm_) "SelfHitTestInvisible"))

(fn `set_black_team_from_array`
  (set `self.black1` (`|GetArrayItem` (`self.black_team(GM)`)))
  (set `self.black2` (`|GetArrayItem` (`self.black_team(GM)`) 1))
  (set `self.black3` (`|GetArrayItem` (`self.black_team(GM)`) 2))
  (set `self.black4` (`|GetArrayItem` (`self.black_team(GM)`) 3))
  (set `self.black5` (`|GetArrayItem` (`self.black_team(GM)`) 4)))

(fn `set_turn_count`
  (set `self.turn_count` (+ (`self.turn_count`) 1)))

(fn `set_white_team_from_array`
  (set `self.white1` (`|GetArrayItem` (`self.white_team(GM)`)))
  (set `self.white2` (`|GetArrayItem` (`self.white_team(GM)`) 1))
  (set `self.white3` (`|GetArrayItem` (`self.white_team(GM)`) 2))
  (set `self.white4` (`|GetArrayItem` (`self.white_team(GM)`) 3))
  (set `self.white5` (`|GetArrayItem` (`self.white_team(GM)`) 4)))

(fn `UserConstructionScript`)

(fn `White Wins`
  (`KismetSystemLibrary.PrintString` "백돌 승리!")
  (`Widget.SetVisibility` (`self.level_UI(gm)`) "Hidden")
  (bind _returnvalue (`|CreateWidget` "/Game/Blueprints/BP_White_Win.BP_White_Win_C"))
  (`UserWidget.AddToViewport` _returnvalue 0))