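; Castle Warrior egg character, a child Blueprint that sets its own health, power and defence on BeginPlay before calling the parent.
; Its skill changes EggState, doubles EggPower, prints the new value and calls EffectOn.
; Skill_Destroy calls EffectOff.
; The Effect_On and Effect_Off events toggle the SkillAura component, with Effect_Off also restoring base power.
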(event `self.ReceiveBeginPlay`
  (set `self.Max Health` 120.0)
  (set `self.Current Health` 120.0)
  (set `self.Egg Power` 14.0)
  (set `self.Skill Damage` 0.0)
  (set `self.Egg Defence` 8.0)
  (`parent.ReceiveBeginPlay`))

(event `self.Egg_Skill`
  (params (Executor :type "/Game/Blueprints/Character/Egg_BlackKnight Object Reference"))
  (set `self.Egg State` "NewEnumerator5")
  (bind _output_get (set `self.Egg Power` 28.0))
  (`KismetSystemLibrary.PrintString` (`KismetStringLibrary.Conv_DoubleToString` _output_get))
  (`self.Effect_On`))

(event `Skill_Destroy`
  (`self.Effect_Off`))

(event `Effect_On`
  (`ActorComponent.Activate` (`self.SkillAura`) false))

(event `Effect_Off`
  (set `self.Egg Power` 14.0)
  (`ActorComponent.Deactivate` (`self.SkillAura`)))

(fn `UserConstructionScript`
  (`parent.UserConstructionScript`))