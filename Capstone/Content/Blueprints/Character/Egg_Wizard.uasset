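; Wizard egg character for an Alkkagi game, a healer that sets its own stats on BeginPlay.
; EggSkill briefly enables SkillCollision, shows range visuals and a heal aura, then advances the game state's turn.
; Healing runs on end overlap, adding SkillDamage as health up to max, only for Egg_BlackKnight actors with a matching first team-style component tag.
; A Heal_Skill spawn is left unconnected.
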(event `self.ReceiveBeginPlay`
  (bind _output_get (set `self.Max Health` 75.0))
  (set `self.Current Health` _output_get)
  (set `self.Egg Power` 12.0)
  (set `self.Skill Damage` 30.0)
  (set `self.Egg Defence` 2.0)
  (`parent.ReceiveBeginPlay`))

(event `self.Egg_Skill`
  (params (Executor :type "/Game/Blueprints/Character/Egg_BlackKnight Object Reference"))
  (`PrimitiveComponent.SetCollisionEnabled` (`self.Skill Collision`) "QueryOnly")
  (`KismetSystemLibrary.Delay` 0.2)
  (`PrimitiveComponent.SetCollisionEnabled` (`self.Skill Collision`) "NoCollision")
  (set `self.Egg State` "NewEnumerator5")
  (`self.Play Skill Effect`)
  (`SceneComponent.SetVisibility` (`self.Skill Range`) true false)
  (`SceneComponent.SetVisibility` (`self.Skill Range2`) true false)
  (`KismetSystemLibrary.Delay` 2.0)
  (`SceneComponent.SetVisibility` (`self.Skill Range`) false false)
  (`SceneComponent.SetVisibility` (`self.Skill Range2`) false false)
  (`/Game/Blueprints/mode/AlkkagiGameStateBase.AddTurn` (cast `/Game/Blueprints/mode/AlkkagiGameStateBase` (`GameplayStatics.GetGameState`) :!pure true)))

(event `self.Skill Collision.OnComponentEndOverlap`
  (params (OverlappedComponent :type "PrimitiveComponent Object Reference") (OtherActor :type "Actor Object Reference") (OtherComp :type "PrimitiveComponent Object Reference") (OtherBodyIndex :type Integer))
  ;[1 1 1] 스킬 콜리전에 엔드 오버랩된 알이 태그가 같으면 체력 회복 / 회복된 체력이 최대 체력을 넘어가면 최대 체력으로 설정
  (bind _asegg_black_knight (cast `/Game/Blueprints/Character/Egg_BlackKnight` OtherActor))
  (if (== (`|GetArrayItem` (`ActorComponent.ComponentTags` (`/Game/Blueprints/Character/Egg_BlackKnight.Egg` _asegg_black_knight))) (`|GetArrayItem` (`ActorComponent.ComponentTags` (`self.Egg`))))
    (bind _current_health (`/Game/Blueprints/Character/Egg_BlackKnight.Current Health` _asegg_black_knight))
    (set `/Game/Blueprints/Character/Egg_BlackKnight.Current Health` (+ _current_health (`self.Skill Damage`)) _asegg_black_knight)
    (bind _max_health (`/Game/Blueprints/Character/Egg_BlackKnight.Max Health` _asegg_black_knight))
    (if (< _max_health _current_health)
      (set `/Game/Blueprints/Character/Egg_BlackKnight.Current Health` _max_health _asegg_black_knight))))

(event `Play Skill Effect`
  (bind _heal_aura (`self.Heal Aura`))
  (`ActorComponent.Activate` _heal_aura false)
  (`KismetSystemLibrary.Delay` 2.0)
  (`ActorComponent.Deactivate` _heal_aura))

(fn `UserConstructionScript`
  (`parent.UserConstructionScript`))