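; Giant Woman guardian egg for a turn-based alkkagi game, setting its own stats, summon type and material.
; Its skill spends owner MP, sets the egg state and advances the turn after a delay.
; A once-gated effect spawns Guardian_Skill and pulses SkillCollision; on end overlap, the server knocks differently tagged Egg_BlackKnight eggs away.
; Timelines lengthen the camera arm and scale the aura during a Niagara disappearance that disables collision.
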(event `self.ReceiveBeginPlay`
  (set `self.Current Health` 65.0)
  (set `self.Max Health` 65.0)
  (set `self.Egg Power` 20.0)
  (set `self.Skill Damage` 10.0)
  (set `self.Egg Defence` 7.0)
  (set `self.Summon Character Type` "/Game/Blueprints/Character/SummonEffect/Blueprints_Summon/BP_Guardian_Summon.BP_Guardian_Summon_C")
  (`self.Guardian Materials Setting`)
  (`parent.ReceiveBeginPlay`))

(event `self.Egg_Skill`
  (params (Executor :type "/Game/Blueprints/Character/Egg_BlackKnight Object Reference"))
  (bind _giantwoman_mp (`self.GiantWoman_MP`))
  (bind _asalkkagi_control (cast `/Game/Blueprints/mode/Alkkagi_Control` (`self.GetOwner`) :!pure true))
  (bind _mp (`/Game/Blueprints/mode/Alkkagi_Control.MP` _asalkkagi_control))
  (if (>= _mp _giantwoman_mp)
    (set `/Game/Blueprints/mode/Alkkagi_Control.Is Shooted` true _asalkkagi_control)
    (set `/Game/Blueprints/mode/Alkkagi_Control.MP` (- _mp _giantwoman_mp) _asalkkagi_control)
    (set `self.Egg State` "NewEnumerator5")
    (`KismetSystemLibrary.Delay` 2.0)
    (`self.Reset Impulse`)
    (`/Game/Blueprints/mode/AlkkagiGameStateBase.AddTurn` (cast `/Game/Blueprints/mode/AlkkagiGameStateBase` (`GameplayStatics.GetGameState`) :!pure true))))

(event `Play Skill Effect`
  (`/Engine/EditorBlueprintResources/StandardMacros.DoOnce` false :!label _label
    (:`Completed`
      (`|SpawnActorFromClass` "/Game/Blueprints/Character/SkillEffect/Guardian_Skill.Guardian_Skill_C" (`KismetMathLibrary.Conv_VectorToTransform` (`SceneComponent.K2_GetComponentLocation` (`self.Character`))) "AlwaysSpawn" "OverrideRootScale" null null)
      (`PrimitiveComponent.SetCollisionEnabled` (`self.Skill Collision`) "QueryOnly")
      (`KismetSystemLibrary.Delay` 0.2)
      (`PrimitiveComponent.SetCollisionEnabled` (`self.Skill Collision`) "NoCollision"))))

(event `Reset Impulse`
  (goto _label :!via `Reset`))

(event `self.Skill Collision.OnComponentEndOverlap`
  (params (OverlappedComponent :type "PrimitiveComponent Object Reference") (OtherActor :type "Actor Object Reference") (OtherComp :type "PrimitiveComponent Object Reference") (OtherBodyIndex :type Integer))
  (bind _egg (`self.Egg`))
  ;[1 1 1] 알의 태그가 다르면 알을 튕겨냄
  (bind _asegg_black_knight (cast `/Game/Blueprints/Character/Egg_BlackKnight` OtherActor))
  (bind _egg_2 (`/Game/Blueprints/Character/Egg_BlackKnight.Egg` _asegg_black_knight))
  (if (!= (`|GetArrayItem` (`ActorComponent.ComponentTags` _egg_2)) (`|GetArrayItem` (`ActorComponent.ComponentTags` _egg)))
    (`/Engine/EditorBlueprintResources/ActorMacros.Switch Has Authority`
      (:`Authority`
        (`PrimitiveComponent.AddImpulse` (`/Game/Blueprints/Character/Egg_BlackKnight.Egg` _asegg_black_knight) (* (- (`SceneComponent.K2_GetComponentLocation` _egg_2) (`SceneComponent.K2_GetComponentLocation` _egg)) 10.0) "None" true)))))

(event `Skill Camera End`
  (bind _springarm (`self.SpringArm`))
  ;[1 1 1] 데미지를 주면서 카메라 거리 증가
  (bind (_direction _spring_arm_length) (`Timeline|타임라인_0_0`)
    (:`Update`
      (set `SpringArmComponent.TargetArmLength` (+ (`SpringArmComponent.TargetArmLength` _springarm) _spring_arm_length) _springarm))))

(event `self.Egg Disappear Niagara`
  (bind _sk_blade_heavyaxe (`self.SK_Blade_HeavyAxe`))
  (bind _character (`self.Character`))
  (bind _aura (`self.Aura`))
  (bind (_returnvalue_location _returnvalue_rotation) (`KismetMathLibrary.BreakTransform` (`SceneComponent.K2_GetComponentToWorld` _character)))
  (bind (_returnvalue_location_2 _returnvalue_rotation_2) (`KismetMathLibrary.BreakTransform` (`SceneComponent.K2_GetComponentToWorld` _sk_blade_heavyaxe)))
  (`KismetSystemLibrary.Delay` 0.5)
  (bind _returnvalue (`NiagaraFunctionLibrary.SpawnSystemAttached` "/Game/Blueprints/Character/Disappear_Niagara/NS_GiantWoman.NS_GiantWoman" _character "None" _returnvalue_location _returnvalue_rotation "KeepRelativeOffset"))
  (bind _returnvalue_2 (`NiagaraFunctionLibrary.SpawnSystemAttached` "/Game/Blueprints/Character/Disappear_Niagara/NS_GiantWoman_Weapon.NS_GiantWoman_Weapon" _sk_blade_heavyaxe "None" _returnvalue_location_2 _returnvalue_rotation_2 "KeepRelativeOffset"))
  (`SceneComponent.SetVisibility` _sk_blade_heavyaxe false false)
  (`SceneComponent.SetVisibility` _character false false)
  (bind (_direction `_새_트랙_1`) (`Timeline|타임라인_0` :!via `PlayFromStart`)
    (:`Update`
      (`SceneComponent.SetRelativeScale3D` _aura `_새_트랙_1`))
    (:`Finished`
      (`SceneComponent.SetVisibility` _aura false false)
      (`ActorComponent.K2_DestroyComponent` _returnvalue)
      (`ActorComponent.K2_DestroyComponent` _returnvalue_2)
      (`PrimitiveComponent.SetCollisionEnabled` (`self.Egg`) "NoCollision"))))

(fn `Guardian Materials Setting`
  (bind _original_materials (`self.Original Materials`))
  (`KismetArrayLibrary.Array_Clear` _original_materials)
  (`KismetArrayLibrary.Array_Add` _original_materials "/Game/Blueprints/Character/GiantWoman/Uriel_MAT.Uriel_MAT"))

(fn `UserConstructionScript`
  (`parent.UserConstructionScript`))