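; BP_Summon_Cube is a summon-effect actor: a cube that rises for the length of a timeline, then destroys itself.
; Each timeline update nudges the actor upward by a fixed, frame-dependent step and writes the cube's world location and scale to the PC_Data Material Parameter Collection as "Position 1" and "Bounds".
; The construction script writes the same parameters, so materials reading the collection have the cube's volume before play.
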(event `self.ReceiveBeginPlay`
  (`Timeline|타임라인_0`
    (:`Update`
      (bind (_sweephitresult _returnvalue) (`self.K2_SetActorLocation` (+ (`self.K2_GetActorLocation`) (0.0 0.0 0.8))))
      (`self.Set Vector Parameters`)
      (if _returnvalue
        _))
    (:`Finished`
      (`self.K2_DestroyActor`)
      (`KismetSystemLibrary.PrintString` "cube destroyed"))))

(event `Set Vector Parameters`
  (bind _cube (`self.Cube`))
  (`KismetMaterialLibrary.SetVectorParameterValue` "/Game/Blueprints/Character/SummonEffect/Materials_Summon/PC_Data.PC_Data" "Position 1" (`KismetMathLibrary.Conv_VectorToLinearColor` (`SceneComponent.K2_GetComponentLocation` _cube)))
  (`KismetMaterialLibrary.SetVectorParameterValue` "/Game/Blueprints/Character/SummonEffect/Materials_Summon/PC_Data.PC_Data" "Bounds" (`KismetMathLibrary.Conv_VectorToLinearColor` (`SceneComponent.K2_GetComponentScale` _cube))))

(fn `UserConstructionScript`
  (bind _cube (`self.Cube`))
  (`KismetMaterialLibrary.SetVectorParameterValue` "/Game/Blueprints/Character/SummonEffect/Materials_Summon/PC_Data.PC_Data" "Position 1" (`KismetMathLibrary.Conv_VectorToLinearColor` (`SceneComponent.K2_GetComponentLocation` _cube)))
  (`KismetMaterialLibrary.SetVectorParameterValue` "/Game/Blueprints/Character/SummonEffect/Materials_Summon/PC_Data.PC_Data" "Bounds" (`KismetMathLibrary.Conv_VectorToLinearColor` (`SceneComponent.K2_GetComponentScale` _cube))))