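; Egg_W is a possessable white-side knight egg unit that aims by click and battles Egg_BlackKnight units.
; While possessed, clicking the egg anchors a cursor trace that rotates it and stretches an arrow by distance; axes control the spring-arm camera.
; Hitting a black knight after a click deducts health, plays attack animations and spawns a crash actor.
; Fire-zone overlaps only set a flag, with separate functions for fire damage and death.
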(event `self.ReceiveUnpossessed`
  (params (OldController :type "Controller Object Reference"))
  (bind _springarm (`self.SpringArm`))
  (set `self.W_possessed` false)
  (`SceneComponent.SetVisibility` (`self.Arrow`) false false)
  (`SkeletalMeshComponent.PlayAnimation` (`self.Knight`) "/Game/Source/Charactor/Animations/Basic_idle.Basic_idle" true)
  (set `SpringArmComponent.TargetArmLength` 1000.0 _springarm)
  (`SceneComponent.K2_SetRelativeRotation` _springarm (struct :`Pitch` -50.0 :`Yaw` -180.0) false false))

(event `self.ReceivePossessed`
  (params (NewController :type "Controller Object Reference"))
  (`SkeletalMeshComponent.PlayAnimation` (`self.Knight`) "/Game/Source/Charactor/Animations/Selected.Selected" true))

(event `self.ReceiveTick`
  (params (DeltaSeconds :type "Float (single-precision)"))
  (if (`self.W_possessed`)
    (`SceneComponent.SetVisibility` (`self.Active`) true false)
    (if (`self.Egg Clicked_W`)
      (`self.Rotate Arrow` (stale `self.Egg.OnClicked` _egg_position)))
    (else
      (`SceneComponent.SetVisibility` (`self.Active`) false false))))

(event `self.Egg.OnClicked`
  (params (TouchedComponent :type "PrimitiveComponent Object Reference") (ButtonPressed :type "Key Structure"))
  (if (`self.W_possessed`)
    (bind _egg_position (`self.Egg Click`))
    (`KismetSystemLibrary.PrintText` (`KismetTextLibrary.Conv_VectorToText` _egg_position))))

(event `self.ReceiveHit`
  (params (MyComp :type "PrimitiveComponent Object Reference") (Other :type "Actor Object Reference") (OtherComp :type "PrimitiveComponent Object Reference") (bSelfMoved :type Boolean) (HitLocation :type "Vector Structure") (HitNormal :type "Vector Structure") (NormalImpulse :type "Vector Structure") (Hit :type "HitResult Structure (by ref)"))
  (bind _returnvalue (`SceneComponent.K2_GetComponentLocation` (`self.Egg`)))
  (if (`self.Egg Clicked_W`)
    (bind _asegg_black_knight (cast `/Game/Blueprints/Character/Egg_BlackKnight` Other))
    (`self.Reduce_Health` _asegg_black_knight)
    (`SkeletalMeshComponent.PlayAnimation` (`/Game/Blueprints/Character/Egg_BlackKnight.Character` _asegg_black_knight) "/Game/Source/Charactor/Animations/Attacked.Attacked" true)
    (`SkeletalMeshComponent.PlayAnimation` (`self.Knight`) "/Game/Source/Charactor/Animations/Slash.Slash" true)
    (set `self.isCrashed_W` true)
    (set `self.CrashPos_W` (+ _returnvalue (0.0 0.0 1500.0)))
    (`|SpawnActorFromClass` "/Game/Blueprints/Crash_Actor.Crash_Actor_C" (`KismetMathLibrary.Conv_VectorToTransform` (+ _returnvalue (0.0 0.0 10.0))) "Undefined" "OverrideRootScale" null null)))

(event `InputAxis|Turn`
  (params (AxisValue :type "Float (single-precision)"))
  (if (`self.W_possessed`)
    (`SceneComponent.K2_AddWorldRotation` (`self.SpringArm`) (`KismetMathLibrary.MakeRotator` 0.0 0.0 AxisValue) false true)))

(event `InputAxis|Zoom`
  (params (AxisValue :type "Float (single-precision)"))
  (bind _springarm (`self.SpringArm`))
  (if (`self.W_possessed`)
    (set `SpringArmComponent.TargetArmLength` (+ (* AxisValue 100.0) (`SpringArmComponent.TargetArmLength` _springarm)) _springarm)))

(event `self.ReceiveActorBeginOverlap`
  (params (OtherActor :type "Actor Object Reference"))
  (bind _returnvalue (`GameplayStatics.GetObjectClass` OtherActor))
  ;[1 1 1] 불장판에 닿으면 health 20 감소, isOnFire를 True로 변경
  (if (or (== _returnvalue "/Game/Blueprints/fire/BP_Fire_Zone_75per.BP_Fire_Zone_75per_C") (== _returnvalue "/Game/Blueprints/fire/BP_Fire_Zone_60per.BP_Fire_Zone_60per_C") (== _returnvalue "/Game/Blueprints/fire/BP_Fire_Zone_50per.BP_Fire_Zone_50per_C") (== _returnvalue "/Game/Blueprints/fire/BP_Fire_Zone_40per.BP_Fire_Zone_40per_C"))
    (set `self.isOnFire(W)` true)))

(event `self.ReceiveActorEndOverlap`
  (params (OtherActor :type "Actor Object Reference"))
  (bind _returnvalue (`GameplayStatics.GetObjectClass` OtherActor))
  ;[1 1 1] 불에서 빠져나오면 isOnFire를 False로 변경
  (if (or (== _returnvalue "/Game/Blueprints/fire/BP_Fire_Zone_75per.BP_Fire_Zone_75per_C") (== _returnvalue "/Game/Blueprints/fire/BP_Fire_Zone_60per.BP_Fire_Zone_60per_C") (== _returnvalue "/Game/Blueprints/fire/BP_Fire_Zone_50per.BP_Fire_Zone_50per_C") (== _returnvalue "/Game/Blueprints/fire/BP_Fire_Zone_40per.BP_Fire_Zone_40per_C"))
    (set `self.isOnFire(W)` false)))

(fn `DestroyEffect`)

(fn `Egg Click`
  (returns (`Egg Position` :type "Vector Structure"))
  (set `self.Egg Clicked_W` true)
  (bind _output_get (set `self.Egg_Pos_W` (`SceneComponent.K2_GetComponentLocation` (`self.Egg`))))
  (return _output_get))

(fn `Reduce_Health`
  (params (`damaged egg` :type "/Game/Blueprints/Character/Egg_BlackKnight Object Reference"))
  (bind _output_get (set `/Game/Blueprints/Character/Egg_BlackKnight.Current Health` (- (`/Game/Blueprints/Character/Egg_BlackKnight.Current Health` `damaged egg`) 20.0) `damaged egg`)))

(fn `Rotate Arrow`
  (params (Egg_Position :type "Vector Structure"))
  (bind (_bblockinghit _binitialoverlap _time _distance _location _impactpoint _normal _impactnormal _physmat _hitactor) (`GameplayStatics.BreakHitResult` (`PlayerController.GetHitResultUnderCursorByChannel` (`GameplayStatics.GetPlayerController` 0) "TraceTypeQuery1" true)))
  (`SceneComponent.SetVisibility` (`self.Arrow`) true false)
  (cast `/Game/Blueprints/Character/Egg_W` _hitactor
    (:`CastFailed`
      (bind _output_get (set `self.Egg_Rotation` (`KismetMathLibrary.Conv_VectorToRotator` (- Egg_Position (`KismetMathLibrary.MakeVector` (.x _location) (.y _location) (.z Egg_Position))))))
      (`SceneComponent.K2_SetWorldRotation` (`self.Egg`) _output_get false false)
      (`SceneComponent.SetWorldScale3D` (`self.Arrow`) (`KismetMathLibrary.MakeVector` (/ (`KismetMathLibrary.Sqrt` (`KismetMathLibrary.DistanceSquared2D` (`KismetMathLibrary.Conv_VectorToVector2D` _location) (`KismetMathLibrary.Conv_VectorToVector2D` Egg_Position))) 60.0) 5.0 5.0)))))

(fn `Set Unit Dead(W)`
  (set `self.isDead(W)` true)
  (`self.SetActorHiddenInGame` true)
  (`self.SetActorEnableCollision` false))

(fn `Take Fire Damage(W)`
  (bind _output_get (set `self.health(W)` (- (`self.health(W)`) 20.0)))
  (set `self.hp_percent(W)` (/ _output_get 100.0)))

(fn `UserConstructionScript`)