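; Archer egg character for the Alkkagi game, a child Blueprint that sets its own health, power, skill damage, defence and summon type on BeginPlay.
; EggSkill spends the owning Alkkagi_Control's MP to spawn one Archer_Range actor at the egg, registering itself as executor.
; The destroy events remove that skill actor and clear the active and selection state.
; On disappearance, a delayed Niagara effect replaces the mesh while a timeline scales the aura before hiding it.
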(event `self.ReceiveBeginPlay`
  (set `self.Max Health` 70.0)
  (set `self.Current Health` 70.0)
  (set `self.Egg Power` 10.0)
  (set `self.Skill Damage` 40.0)
  (set `self.Egg Defence` 3.0)
  (set `self.Summon Character Type` "/Game/Blueprints/Character/SummonEffect/Blueprints_Summon/BP_Archer_Summon.BP_Archer_Summon_C")
  (`parent.ReceiveBeginPlay`))

(event `self.Egg_Skill`
  (params (Executor :type "/Game/Blueprints/Character/Egg_BlackKnight Object Reference"))
  (bind _archer_mp (`self.Archer_MP`))
  (bind _asalkkagi_control (cast `/Game/Blueprints/mode/Alkkagi_Control` (`self.GetOwner`) :!pure true))
  (bind _mp (`/Game/Blueprints/mode/Alkkagi_Control.MP` _asalkkagi_control))
  (`/Engine/EditorBlueprintResources/StandardMacros.IsValid` (`self.Skill Actor`)
    (:`Is Not Valid`
      (if (>= _mp _archer_mp)
        (set `/Game/Blueprints/mode/Alkkagi_Control.MP` (- _mp _archer_mp) _asalkkagi_control)
        (bind _returnvalue (`|SpawnActorFromClass` "/Game/Blueprints/Character/SkillEffect/Archer_Range.Archer_Range_C" (`SceneComponent.K2_GetComponentToWorld` (`self.Egg`)) "AlwaysSpawn" "OverrideRootScale" (`self.GetOwner`) null))
        (bind _output_get (set `self.Skill Actor` _returnvalue))
        (set `/Game/Blueprints/Character/SkillEffect/Archer_Range.Executor Egg` self _output_get)))))

(event `Skill_Destroy`
  (`self.Destroy`))

(event `Destroy`
  (`self.K2_DestroyActor` (`self.Skill Actor`))
  (`SceneComponent.SetVisibility` (`self.Active`) false false)
  (set `self.possessed` false)
  (set `self.Egg Clicked` false))

(event `self.Egg Disappear Niagara`
  (bind _character (`self.Character`))
  (bind _aura (`self.Aura`))
  (bind (_returnvalue_location _returnvalue_rotation) (`KismetMathLibrary.BreakTransform` (`SceneComponent.K2_GetComponentToWorld` _character)))
  (`KismetSystemLibrary.Delay` 0.5)
  (bind _returnvalue (`NiagaraFunctionLibrary.SpawnSystemAttached` "/Game/Blueprints/Character/Disappear_Niagara/NS_Archer.NS_Archer" _character "None" _returnvalue_location _returnvalue_rotation "KeepRelativeOffset"))
  (`SceneComponent.SetVisibility` _character false false)
  (bind (_direction `_새_트랙_1`) (`Timeline|타임라인_0` :!via `PlayFromStart`)
    (:`Update`
      (`SceneComponent.SetRelativeScale3D` _aura `_새_트랙_1`))
    (:`Finished`
      (`SceneComponent.SetVisibility` _aura false false)
      (`ActorComponent.K2_DestroyComponent` _returnvalue))))

(fn `UserConstructionScript`
  (`parent.UserConstructionScript`))