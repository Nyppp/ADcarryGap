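; Black Knight egg for a turn-based Alkkagi flicking game, with replication, health and death handling.
; Slingshot aiming rotates and stretches an arrow from the cursor, then launches the egg with a capped impulse; egg collisions go to AlkkagiGameStateBase.
; Its skill briefly enables a collision volume, damaging differently tagged Black Knight eggs on end overlap, then advances the turn.
; Fire zone overlaps toggle IsOnFire, with a separate function applying burn damage.
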(event `self.ReceiveBeginPlay`
  ;[1 1 1] 딜레이 후 리플리케이션 설정
  (`KismetSystemLibrary.Delay` 0.5)
  (`ActorComponent.SetIsReplicated` (`self.Egg`) true)
  (`ActorComponent.SetIsReplicated` (`self.ProjectileMovement`) true)
  (`PrimitiveComponent.SetCollisionEnabled` (`self.Skill Collision`) "NoCollision"))

(event `self.ReceiveHit`
  (params (MyComp :type "PrimitiveComponent Object Reference") (Other :type "Actor Object Reference") (OtherComp :type "PrimitiveComponent Object Reference") (bSelfMoved :type Boolean) (HitLocation :type "Vector Structure") (HitNormal :type "Vector Structure") (NormalImpulse :type "Vector Structure") (Hit :type "HitResult Structure (by ref)"))
  ;[1 1 1] 알이 부딪힐 시 게임 스테이트에서 에그 히트 이벤트 실행
  (bind _asegg_black_knight (cast `/Game/Blueprints/Character/Egg_BlackKnight` Other))
  (`/Game/Blueprints/mode/AlkkagiGameStateBase.EggHit` (cast `/Game/Blueprints/mode/AlkkagiGameStateBase` (`GameplayStatics.GetGameState`) :!pure true) self _asegg_black_knight))

(event `self.ReceiveAnyDamage`
  (params (Damage :type "Float (single-precision)") (DamageType :type "DamageType Object Reference") (InstigatedBy :type "Controller Object Reference") (DamageCauser :type "Actor Object Reference"))
  ;[1 1 1] 데미지를 받았을 경우 데미지만큼 체력 감소
  (bind _output_get (set `self.Current Health` (- (`self.Current Health`) Damage)))
  (if (<= _output_get 0.0)
    (`self.K2_DestroyActor`)))

(event `self.ReceiveActorBeginOverlap`
  (params (OtherActor :type "Actor Object Reference"))
  (bind _returnvalue (`GameplayStatics.GetObjectClass` OtherActor))
  ;[1 1 1] 불장판에 닿으면 health 20 감소, isOnFire를 True로 변경
  (if (or (== _returnvalue "/Game/Blueprints/fire/BP_Fire_Zone_75per.BP_Fire_Zone_75per_C") (== _returnvalue "/Game/Blueprints/fire/BP_Fire_Zone_60per.BP_Fire_Zone_60per_C") (== _returnvalue "/Game/Blueprints/fire/BP_Fire_Zone_50per.BP_Fire_Zone_50per_C") (== _returnvalue "/Game/Blueprints/fire/BP_Fire_Zone_40per.BP_Fire_Zone_40per_C"))
    (set `self.Is OnFire` true)))

(event `self.ReceiveActorEndOverlap`
  (params (OtherActor :type "Actor Object Reference"))
  (bind _returnvalue (`GameplayStatics.GetObjectClass` OtherActor))
  ;[1 1 1] 불에서 빠져나오면 isOnFire를 False로 변경
  (if (or (== _returnvalue "/Game/Blueprints/fire/BP_Fire_Zone_75per.BP_Fire_Zone_75per_C") (== _returnvalue "/Game/Blueprints/fire/BP_Fire_Zone_60per.BP_Fire_Zone_60per_C") (== _returnvalue "/Game/Blueprints/fire/BP_Fire_Zone_50per.BP_Fire_Zone_50per_C") (== _returnvalue "/Game/Blueprints/fire/BP_Fire_Zone_40per.BP_Fire_Zone_40per_C"))
    (set `self.Is OnFire` false)))

(event `Egg_Skill`
  (params (Executor :type "/Game/Blueprints/Character/Egg_BlackKnight Object Reference"))
  ;[1 1 1] 캐릭터 스킬
  (set `self.Egg State` "NewEnumerator5")
  (`PrimitiveComponent.SetCollisionEnabled` (`self.Skill Collision`) "QueryOnly")
  (`KismetSystemLibrary.Delay` 0.2)
  (`PrimitiveComponent.SetCollisionEnabled` (`self.Skill Collision`) "NoCollision")
  (`KismetSystemLibrary.PrintString` "블랙워리어 스킬")
  (`KismetSystemLibrary.Delay` 1.2)
  (`/Game/Blueprints/mode/AlkkagiGameStateBase.AddTurn` (cast `/Game/Blueprints/mode/AlkkagiGameStateBase` (`GameplayStatics.GetGameState`) :!pure true)))

(event `self.Skill Collision.OnComponentEndOverlap`
  (params (OverlappedComponent :type "PrimitiveComponent Object Reference") (OtherActor :type "Actor Object Reference") (OtherComp :type "PrimitiveComponent Object Reference") (OtherBodyIndex :type Integer))
  ;[1 1 1] 코멘트
  (bind _asegg_black_knight (cast `/Game/Blueprints/Character/Egg_BlackKnight` OtherActor))
  (if (!= (`|GetArrayItem` (`ActorComponent.ComponentTags` (`/Game/Blueprints/Character/Egg_BlackKnight.Egg` _asegg_black_knight))) (`|GetArrayItem` (`ActorComponent.ComponentTags` (`self.Egg`))))
    (`GameplayStatics.ApplyDamage` _asegg_black_knight (`self.Skill Damage`))))

(event `self.ProjectileMovement.OnProjectileStop`
  (params (ImpactResult :type "HitResult Structure (by ref)"))
  (`KismetSystemLibrary.PrintString` "Hello"))

(fn `Character Skill`)

(fn `Egg Click`
  (set `self.Egg Clicked` true)
  (set `self.Egg Pos` (`SceneComponent.K2_GetComponentLocation` (`self.Egg`)))
  (return))

(fn `Egg Shoot`
  (params (`Mouse Pos` :type "Vector Structure"))
  (bind _returnvalue (`SceneComponent.K2_GetComponentLocation` (`self.Egg`)))
  (bind _returnvalue_2 (* (`KismetMathLibrary.MakeVector` (.x (- _returnvalue `Mouse Pos`)) (.y (- _returnvalue `Mouse Pos`)) (.z _returnvalue)) 3))
  (bind _returnvalue_3 (`KismetMathLibrary.VSize` _returnvalue_2))
  (`SceneComponent.SetVisibility` (`self.Arrow`) false true)
  (if (< _returnvalue_3 2000.0)
    (`PrimitiveComponent.AddImpulse` (`self.Egg`) _returnvalue_2 "None" true)
    (set `self.possessed` false)
    (else
      (`PrimitiveComponent.AddImpulse` (`self.Egg`) (* (/ _returnvalue_2 _returnvalue_3) 2000.0) "None" true)
      (set `self.possessed` false))))

(fn `Re Impulse`
  (params (`Egg Power` :type "Vector Structure"))
  (`PrimitiveComponent.AddImpulse` (`self.Egg`) `Egg Power` "None" true))

(fn `Rotate Arrow`
  (params (`Egg Position` :type "Vector Structure") (`Mouse Position` :type "Vector Structure"))
  (bind _returnvalue (`KismetMathLibrary.Sqrt` (`KismetMathLibrary.DistanceSquared2D` (`KismetMathLibrary.Conv_VectorToVector2D` `Mouse Position`) (`KismetMathLibrary.Conv_VectorToVector2D` `Egg Position`))))
  (`SceneComponent.SetVisibility` (`self.Arrow`) true false)
  (cast `/Game/Blueprints/Character/Egg_BlackKnight` (`.HitActor` (`GameplayStatics.BreakHitResult` (`PlayerController.GetHitResultUnderCursorByChannel` (`GameplayStatics.GetPlayerController` 0) "TraceTypeQuery1" true)))
    (:`CastFailed`
      (bind _output_get (set `self.Egg Rotation` (`KismetMathLibrary.Conv_VectorToRotator` (- `Egg Position` (`KismetMathLibrary.MakeVector` (.x `Mouse Position`) (.y `Mouse Position`) (.z `Egg Position`))))))
      (`SceneComponent.K2_SetWorldRotation` (`self.Egg`) _output_get false false)
      (if (< _returnvalue 500.0)
        (`SceneComponent.SetWorldScale3D` (`self.Arrow`) (`KismetMathLibrary.MakeVector` (/ _returnvalue 60.0) 5.0 5.0))
        (else
          (`SceneComponent.SetWorldScale3D` (`self.Arrow`) (`KismetMathLibrary.MakeVector` (/ 500.0 60.0) 5.0 5.0)))))))

(fn `Set Unit Dead(B)`
  (set `self.Is Dead` true)
  (`self.SetActorHiddenInGame` true)
  (`self.SetActorEnableCollision` false))

(fn `Take Fire Damage(B)`
  (set `self.Current Health` (- (`self.Current Health`) 20.0)))

(fn `UserConstructionScript`)