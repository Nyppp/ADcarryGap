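; BP_BGM_Player is an actor that plays the game's background music through a single Audio component.
; PlayBGM stops the current track, swaps in the sound it is given and restarts playback from the beginning.
; PlayResultBGM compares HostIsWinner with IsServer to tell whether the local side won, then plays the News Theme cue for a win or the Quiet cue for a loss.
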(event `self.ReceiveBeginPlay`)

(fn `Play BGM`
  (params (`New BGM` :type "SoundCue Object Reference"))
  (bind _audio (`self.Audio`))
  (`AudioComponent.Stop` _audio)
  (`AudioComponent.SetSound` _audio `New BGM`)
  (`AudioComponent.Play` _audio 0.0))

(fn `Play Result BGM`
  (params (`Host Is Winner` :type Boolean))
  (bind _audio (`self.Audio`))
  (bind _audio_2 (`self.Audio`))
  (if (== `Host Is Winner` (`KismetSystemLibrary.IsServer`))
    (`AudioComponent.Stop` _audio_2)
    (`AudioComponent.SetSound` _audio_2 "/Game/Source/Sounds/BGM/News_Theme_-_Kevin_MacLeod_Cue.News_Theme_-_Kevin_MacLeod_Cue")
    (`AudioComponent.Play` _audio_2 0.0)
    (else
      (`AudioComponent.Stop` _audio)
      (`AudioComponent.SetSound` _audio "/Game/Source/Sounds/BGM/Quiet_-_Audionautix_Cue.Quiet_-_Audionautix_Cue")
      (`AudioComponent.Play` _audio 0.0))))

(fn `UserConstructionScript`)