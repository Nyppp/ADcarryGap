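; Game state for a two-player networked Alkkagi egg-flicking battle, running turns, combat and the match result.
; BeginPlay takes eggs and controllers from the game mode, then sets up team materials, cameras, UI and BGM.
; A gated countdown calls AddTurn on timeout, which flips egg states by turn parity and checks whether either side is wiped out.
; Shots follow a timeline spring-arm zoom; enemy hits trigger a pause, server-side re-impulse and damage.
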(event `State_Shoot`
  (params (`Selected Egg` :type "/Game/Blueprints/Character/Egg_BlackKnight Object Reference") (`Mouse Pos` :type "Vector Structure"))
  (bind _springarm (`/Game/Blueprints/Character/Egg_BlackKnight.SpringArm` `Selected Egg`))
  ;[1 1 1] 스프링암 길이, 각도 조정 후 스테이트 슛
  (bind (_direction _spring_arm_length _spring_arm_y_rotation) (`Timeline|Setting Spring Arm` :!via `PlayFromStart`)
    (:`Update`
      (if (and (`self.Length Condition`) (`self.Rotate Condition`))
        (`self.Setting Spring Arm__Stop Timer__EventFunc`)
        (else
          (`|ExecutionSequence`
            (:`then_0`
              (bind _returnvalue (- (`SpringArmComponent.TargetArmLength` _springarm) _spring_arm_length))
              (if (>= _returnvalue 400.0)
                (set `SpringArmComponent.TargetArmLength` _returnvalue _springarm)
                (else
                  (set `SpringArmComponent.TargetArmLength` 400.0 _springarm)
                  (set `self.Length Condition` true))))
            (:`then_1`
              (bind _returnvalue_2 (+ (.pitch (`SceneComponent.RelativeRotation` _springarm)) _spring_arm_y_rotation))
              (if (>= _returnvalue_2 -35.0)
                (set `self.Rotate Condition` true)
                (else
                  (`/Engine/EditorBlueprintResources/ActorMacros.Switch Has Authority`
                    (:`Authority`
                      (`SceneComponent.K2_SetRelativeRotation` _springarm (`KismetMathLibrary.MakeRotator` 0.0 _returnvalue_2 (.yaw (`/Game/Blueprints/Character/Egg_BlackKnight.Egg Rotation` `Selected Egg`))) false false))))))))))
    (:`Finished`
      (set `self.Length Condition` false)
      (set `self.Rotate Condition` false)
      (`/Engine/EditorBlueprintResources/ActorMacros.Switch Has Authority`
        (:`Authority`
          (`/Game/Blueprints/Character/Egg_BlackKnight.Egg Shoot` `Selected Egg` `Mouse Pos`))))
    (:`Stop Timer`
      (`self.Close Timer Gate`))))

(event `self.ReceiveTick`
  (params (DeltaSeconds :type "Float (single-precision)")))

(event `Play Turn Timer`
  ;[1 1 1] 턴 남은시간을 매초 1씩 감소
  (`/Engine/EditorBlueprintResources/StandardMacros.Gate` true :!label _label
    (:`Exit`
      (`KismetSystemLibrary.Delay` 1.0)
      (`self.Play Turn Timer`)
      (bind _result (`/Engine/EditorBlueprintResources/StandardMacros.DecrementInt` (`self.TurnTimer`))
        (:`  `
          (set `/Game/Blueprints/widget/WB_Level_UI.TurnTimer(LevelUI)` _result (`self.BattleLevelUI`))
          (if (== _result 0)
            (`KismetSystemLibrary.PrintString` "Time Over")
            ;[1 1 1] 턴 남은시간이 0이면 서버에서 AddTurn 호출
            (if (`KismetSystemLibrary.IsServer`)
              (`self.AddTurn`))
            ;[1 1 1] Unpossess
            (bind _asalkkagi_control (cast `/Game/Blueprints/mode/Alkkagi_Control` (`GameplayStatics.GetPlayerController` 0)))
            (`/Game/Blueprints/mode/Alkkagi_Control.UnPossessed` _asalkkagi_control (`/Game/Blueprints/mode/Alkkagi_Control.Selected Egg` _asalkkagi_control))
            (`self.CameraSet` 1.0)))))))

(event `Open Timer Gate`
  ;[1 1 1] 턴 남은시간을 매초 1씩 감소
  (`|ExecutionSequence`
    (:`then_0`
      (goto _label :!via `Open`))
    (:`then_1`
      (`self.Play Turn Timer`))))

(event `Close Timer Gate`
  ;[1 1 1] 턴 남은시간을 매초 1씩 감소
  (goto _label :!via `Close`))

(event `ServerSetEggSpeed`
  (params (`Selected Egg` :type "/Game/Blueprints/Character/Egg_BlackKnight Object Reference") (`Egg Speed` :type "Float (double-precision)"))
  ;[1 1 1] 서버와 클라이언트 모두 선택된 알의 속도를 설정
  (`self.StateSetEggSpeed` `Selected Egg` `Egg Speed`))

(event `AddTurn`
  (bind _battlelevelui (`self.BattleLevelUI`))
  (bind _asalkkagi_gamemode (cast `/Game/Blueprints/mode/Alkkagi_Gamemode` (`GameplayStatics.GetGameMode`) :!pure true))
  ;[1 1 1] 턴 넘어갈 때 턴 카운트 변수 증가 / 턴제 관련해서 이 이벤트 묶어 쓰면 됨
  (bind _result (`/Engine/EditorBlueprintResources/StandardMacros.IncrementInt` (`self.TurnNum`))
    (:`  `
      (set `/Game/Blueprints/widget/WB_Level_UI.TurnCount(LevelUI)` _result (`self.BattleLevelUI`))
      (`self.Change State` (`/Game/Blueprints/mode/Alkkagi_Gamemode.Host Eggs` _asalkkagi_gamemode) (`/Game/Blueprints/mode/Alkkagi_Gamemode.Client Eggs` _asalkkagi_gamemode))
      (`self.CameraSet` 1.0)
      ;[1 1 1] 유닛 생존여부 검사
      (`self.Check Units Survival`)
      ;[1 1 1] 턴 남은시간을 20으로 리셋
      (set `self.TurnTimer` 21)
      ;[1 1 1] UI에 표시할 현재턴 소유자 설정(턴수가 홀수이면 서버, 짝수이면 클라이언트), 추후 플레이어 네임으로 변경
      (switch `int` (mod (`self.TurnNum`) 2)
        (:`0`
          (set `/Game/Blueprints/widget/WB_Level_UI.TurnOwner` "Client" _battlelevelui))
        (:`1`
          (set `/Game/Blueprints/widget/WB_Level_UI.TurnOwner` "Server" _battlelevelui)))
      (`self.Open Timer Gate`))))

(event `StateSetEggSpeed`
  (params (`Selected Egg` :type "/Game/Blueprints/Character/Egg_BlackKnight Object Reference") (`Egg Speed` :type "Float (double-precision)"))
  ;[1 1 1] 서버와 클라이언트 모두 선택된 알의 속도를 설정
  (if true
    (`/Engine/EditorBlueprintResources/ActorMacros.Switch Has Authority`
      (:`Authority`
        (set `/Game/Blueprints/Character/Egg_BlackKnight.Egg Speed` `Egg Speed` `Selected Egg`)))))

(event `Change State`
  (params (`Host Eggs` :type "Array of /Game/Blueprints/Character/Egg_BlackKnight Object Reference") (`Client Eggs` :type "Array of /Game/Blueprints/Character/Egg_BlackKnight Object Reference"))
  ;[1 1 1] 알의 상태 전환
  (for _array_element `Host Eggs`
    (switch `int` (mod (`self.TurnNum`) 2)
      (:`0`
        (set `/Game/Blueprints/Character/Egg_BlackKnight.Egg State` "NewEnumerator2" _array_element))
      (:`1`
        (set `/Game/Blueprints/Character/Egg_BlackKnight.Egg State` "NewEnumerator0" _array_element)))
    (bind _springarm (`/Game/Blueprints/Character/Egg_BlackKnight.SpringArm` _array_element))
    (set `SpringArmComponent.TargetArmLength` 1000.0 _springarm)
    (`SceneComponent.K2_SetRelativeRotation` _springarm (struct :`Pitch` -50.0) false false)
    (`/Game/Blueprints/mode/Alkkagi_Control.UnPossessed` (cast `/Game/Blueprints/mode/Alkkagi_Control` (`self.Host Controller`) :!pure true) _array_element)
    (goto _label_2 :!via `Reset`))
  (for _array_element_2 `Client Eggs`
    (switch `int` (mod (`self.TurnNum`) 2)
      (:`0`
        (set `/Game/Blueprints/Character/Egg_BlackKnight.Egg State` "NewEnumerator0" _array_element_2))
      (:`1`
        (set `/Game/Blueprints/Character/Egg_BlackKnight.Egg State` "NewEnumerator2" _array_element_2)))
    (bind _springarm_2 (`/Game/Blueprints/Character/Egg_BlackKnight.SpringArm` _array_element_2))
    (set `SpringArmComponent.TargetArmLength` 1000.0 _springarm_2)
    (`SceneComponent.K2_SetRelativeRotation` _springarm_2 (struct :`Pitch` -50.0 :`Yaw` 180.0) false false)
    (`/Game/Blueprints/mode/Alkkagi_Control.UnPossessed` (cast `/Game/Blueprints/mode/Alkkagi_Control` (`self.Client Controller`) :!pure true) _array_element_2)
    (goto _label_2 :!via `Reset`)))

(event `Notify Server Re Impulse`
  (params (`My Egg` :type "/Game/Blueprints/Character/Egg_BlackKnight Object Reference") (`Other Egg` :type "/Game/Blueprints/Character/Egg_BlackKnight Object Reference") (`Egg Power` :type "Vector Structure"))
  (bind _egg (`/Game/Blueprints/Character/Egg_BlackKnight.Egg` `Other Egg`))
  (bind _egg_2 (`/Game/Blueprints/Character/Egg_BlackKnight.Egg` `My Egg`))
  ;[1 1 1] 상대편 알에 히트되었을 경우 정지 - 재발사 이벤트
  (`/Engine/EditorBlueprintResources/ActorMacros.Switch Has Authority`
    (:`Authority`
      (`SceneComponent.SetMobility` _egg_2 "Stationary")
      (`SceneComponent.SetMobility` _egg "Stationary")
      (`KismetSystemLibrary.Delay` 0.5)
      (`SceneComponent.SetMobility` _egg_2 "Movable")
      (`SceneComponent.SetMobility` _egg "Movable")
      (`self.State Re Impulse` `My Egg` `Other Egg` `Egg Power`))))

(event `State Re Impulse`
  (params (`My Egg` :type "/Game/Blueprints/Character/Egg_BlackKnight Object Reference") (`Other Egg` :type "/Game/Blueprints/Character/Egg_BlackKnight Object Reference") (`Egg Power` :type "Vector Structure"))
  ;[1 1 1] 상대편 알에 히트되었을 경우 정지 - 재발사 이벤트
  (`/Engine/EditorBlueprintResources/StandardMacros.DoOnce` false :!label _label_2
    (:`Completed`
      (`/Engine/EditorBlueprintResources/ActorMacros.Switch Has Authority`
        (:`Authority`
          (set `/Game/Blueprints/Character/Egg_BlackKnight.Egg State` "NewEnumerator4" `Other Egg`)
          (`KismetSystemLibrary.Delay` 1.0)
          (set `/Game/Blueprints/Character/Egg_BlackKnight.Egg State` "NewEnumerator3" `My Egg`)
          (`/Game/Blueprints/Character/Egg_BlackKnight.Re Impulse` `My Egg` `Egg Power`)
          (goto _label_4 :!via `Reset`))))))

(event `EggHit`
  (params (`My Egg` :type "/Game/Blueprints/Character/Egg_BlackKnight Object Reference") (`Other Egg` :type "/Game/Blueprints/Character/Egg_BlackKnight Object Reference"))
  (bind _springarm (`/Game/Blueprints/Character/Egg_BlackKnight.SpringArm` `My Egg`))
  (bind _springarm_2 (`/Game/Blueprints/Character/Egg_BlackKnight.SpringArm` `My Egg`))
  (bind _egg_power (`/Game/Blueprints/Character/Egg_BlackKnight.Egg Power` `Other Egg`))
  (bind _yaw (.yaw (`/Game/Blueprints/Character/Egg_BlackKnight.Egg Rotation` `My Egg`)))
  (bind _returnvalue (mod (`self.TurnNum`) 2))
  (bind _output (`|GetArrayItem` (`ActorComponent.ComponentTags` (`/Game/Blueprints/Character/Egg_BlackKnight.Egg` `My Egg`))))
  ;[1 1 1] 자신의 알이 상대 알에 히트하면 화면 확대
  (if (`/Game/Blueprints/Character/Egg_BlackKnight.Egg Clicked` `My Egg`)
    (`self.Mana_Charge` `My Egg`)
    (set `/Game/Blueprints/Character/Egg_BlackKnight.Egg State` "NewEnumerator0" `My Egg`)
    (if (!= (`|GetArrayItem` (`ActorComponent.ComponentTags` (`/Game/Blueprints/Character/Egg_BlackKnight.Egg` `My Egg`))) (`|GetArrayItem` (`ActorComponent.ComponentTags` (`/Game/Blueprints/Character/Egg_BlackKnight.Egg` `Other Egg`))))
      (set `SpringArmComponent.TargetArmLength` 400.0 _springarm_2)
      (`/Engine/EditorBlueprintResources/ActorMacros.Switch Has Authority`
        (:`Authority`
          (`SceneComponent.K2_SetRelativeRotation` _springarm_2 (`KismetMathLibrary.MakeRotator` 0.0 -30.0 (.yaw (`/Game/Blueprints/Character/Egg_BlackKnight.Egg Rotation` `My Egg`))) false false))))
    (elif (!= _output (`|GetArrayItem` (`ActorComponent.ComponentTags` (`/Game/Blueprints/Character/Egg_BlackKnight.Egg` `Other Egg`))))
      (set `SpringArmComponent.TargetArmLength` 400.0 _springarm)
      (if (== _output "Host")
        (if (== _returnvalue 0)
          (`SceneComponent.K2_SetRelativeRotation` _springarm (`KismetMathLibrary.MakeRotator` 0.0 -30.0 _yaw) false false)
          (`/Game/Blueprints/mode/Alkkagi_Control.HitZoom` (cast `/Game/Blueprints/mode/Alkkagi_Control` (`self.Host Controller`) :!pure true) `My Egg`)
          (`self.Notify Server Re Impulse` `My Egg` `Other Egg` (* (`KismetMathLibrary.GetForwardVector` (`/Game/Blueprints/Character/Egg_BlackKnight.Egg Rotation` `Other Egg`)) (* _egg_power 100.0)) :!label _label_3)
          (`/Engine/EditorBlueprintResources/StandardMacros.DoOnce` false :!label _label_4
            (:`Completed`
              (`GameplayStatics.ApplyDamage` `My Egg` (- _egg_power (`/Game/Blueprints/Character/Egg_BlackKnight.Egg Defence` `My Egg`)) null `Other Egg`))))
        (elif (== _returnvalue 1)
          (`SceneComponent.K2_SetRelativeRotation` _springarm (`KismetMathLibrary.MakeRotator` 0.0 -30.0 _yaw) false false)
          (`/Game/Blueprints/mode/Alkkagi_Control.HitZoom` (cast `/Game/Blueprints/mode/Alkkagi_Control` (`self.Client Controller`) :!pure true) `My Egg`)
          (goto _label_3))))))

(event `Show Result`
  (params (Winner :type Boolean))
  (bind _returnvalue (`GameplayStatics.GetPlayerController` 0))
  ;[1 1 1] 결과 UI 출력
  (`|ExecutionSequence`
    (:`then_0`
      (`Widget.SetVisibility` (`self.BattleLevelUI`) "Hidden"))
    (:`then_1`
      ;;[1 1 1] Winner가 True이면 서버, False이면 클라이언트 승리
      (if Winner
        (bind _returnvalue_2 (`|CreateWidget` "/Game/Blueprints/widget/WB_Result_Screen.WB_Result_Screen_C" _returnvalue))
        (bind _resulttext (`/Game/Blueprints/widget/WB_Result_Screen.ResultText` _returnvalue_2))
        (`TextBlock.SetText` _resulttext (`KismetTextLibrary.Conv_StringToText` (`KismetStringLibrary.Concat_StrStr` "SERVER" "WIN!")))
        (`TextBlock.SetColorAndOpacity` _resulttext (make `SlateColor` (struct :`A` 1.0)))
        (`UserWidget.AddToViewport` _returnvalue_2 0)
        (else
          (bind _returnvalue_3 (`|CreateWidget` "/Game/Blueprints/widget/WB_Result_Screen.WB_Result_Screen_C" _returnvalue))
          (bind _resulttext_2 (`/Game/Blueprints/widget/WB_Result_Screen.ResultText` _returnvalue_3))
          (`TextBlock.SetText` _resulttext_2 (`KismetTextLibrary.Conv_StringToText` (`KismetStringLibrary.Concat_StrStr` "CLIENT  " "WIN!")))
          (`TextBlock.SetColorAndOpacity` _resulttext_2 (make `SlateColor` (struct :`R` 1.0 :`G` 1.0 :`B` 1.0 :`A` 1.0)))
          (`UserWidget.AddToViewport` _returnvalue_3 0))))))

(event `Mana_Charge`
  (params (Egg :type "/Game/Blueprints/Character/Egg_BlackKnight Object Reference"))
  (bind _asalkkagi_control (cast `/Game/Blueprints/mode/Alkkagi_Control` (`self.GetOwner` Egg) :!pure true))
  (bind _returnvalue (+ (`/Game/Blueprints/mode/Alkkagi_Control.MP` _asalkkagi_control) 10))
  (if (> _returnvalue 100)
    (set `/Game/Blueprints/mode/Alkkagi_Control.MP` 100 _asalkkagi_control)
    (else
      (set `/Game/Blueprints/mode/Alkkagi_Control.MP` _returnvalue _asalkkagi_control))))

(event `Play BGM`
  ;[1 1 1] 대전 국면(초반/중반/후반)에 따라 BGM 재생, 재생 완료시 다시 재생
  (switch `int` (`self.BattlePhase`)
    (:`Default`
      _)
    (:`1`
      _))
  (`GameplayStatics.PlaySound2D` "/Game/Source/Sounds/BGM/battleThemeA.battleThemeA" 0.4 0.85 0.0 null null)
  (`KismetSystemLibrary.Delay` (* 96.0 (/ 1.0 0.85)))
  (`self.Play BGM`))

(event `디버그버튼1`
  (`self.호스트 몰살`))

(event `호스트 몰살`
  (`/Engine/EditorBlueprintResources/ActorMacros.Switch Has Authority`
    (:`Authority`
      (`KismetSystemLibrary.PrintString` "kill")
      (for _array_element (`self.HostEggs`)
        (set `/Game/Blueprints/Character/Egg_BlackKnight.Current Health` 0.0 _array_element)
        (`self.AddTurn`)))))

(event `self.ReceiveBeginPlay`
  (`self.Initial Set1`)
  (`KismetSystemLibrary.Delay` 0.3)
  (bind _returnvalue (`|CreateWidget` "/Game/Blueprints/widget/MultiPlay/Menu/WB_LoadingMenu.WB_LoadingMenu_C" (`GameplayStatics.GetPlayerController` 0)))
  (`UserWidget.AddToViewport` _returnvalue 0)
  (`KismetSystemLibrary.Delay` 1.5)
  (`Widget.RemoveFromParent` _returnvalue)
  (`self.Open Timer Gate`))

(event `Initial Set1`
  ;[1 1 1] 초기 카메라 셋업
  (`KismetSystemLibrary.Delay` 1.5)
  (bind _outactors (`GameplayStatics.GetAllActorsOfClassWithTag` "/Script/Engine.CameraActor" "Host"))
  (`KismetArrayLibrary.Array_Add` (`self.Cameras`) (`|GetArrayItem` _outactors))
  (bind _outactors_2 (`GameplayStatics.GetAllActorsOfClassWithTag` "/Script/Engine.CameraActor" "Client"))
  (`KismetArrayLibrary.Array_Add` (`self.Cameras`) (`|GetArrayItem` _outactors_2))
  (`self.CameraSet` 0.0)
  (`self.Initial Set2`))

(event `Initial Set2`
  ;[1 1 1] UI를 변수로 승격
  (bind _returnvalue (`|CreateWidget` "/Game/Blueprints/widget/WB_Level_UI.WB_Level_UI_C" (`GameplayStatics.GetPlayerController` 0)))
  (`UserWidget.AddToViewport` _returnvalue 0)
  (bind _output_get (set `self.BattleLevelUI` _returnvalue))
  ;[1 1 1] UI에 표시할 실행권한(서버/클라) 표기 설정
  (if (`KismetSystemLibrary.IsServer`)
    (set `/Game/Blueprints/widget/WB_Level_UI.Authority` "SERVER" _output_get)
    (else
      (set `/Game/Blueprints/widget/WB_Level_UI.Authority` "CLIENT" _output_get)))
  (`self.Initial Set3`))

(event `Initial Set3`
  ;[1 1 1] GameMode에서 유닛 배열을 받아옴
  (bind _asalkkagi_gamemode (cast `/Game/Blueprints/mode/Alkkagi_Gamemode` (`GameplayStatics.GetGameMode`)))
  (bind _output_get (set `self.HostEggs` (`/Game/Blueprints/mode/Alkkagi_Gamemode.Host Eggs` _asalkkagi_gamemode)))
  (bind _output_get_2 (set `self.ClientEggs` (`/Game/Blueprints/mode/Alkkagi_Gamemode.Client Eggs` _asalkkagi_gamemode)))
  (`self.EggsSettings` _output_get _output_get_2)
  (bind _allplayercontrollers (`/Game/Blueprints/mode/Alkkagi_Gamemode.AllPlayerControllers` _asalkkagi_gamemode))
  (set `self.Host Controller` (`|GetArrayItem` _allplayercontrollers))
  (set `self.Client Controller` (`|GetArrayItem` _allplayercontrollers 1))
  (`self.Play Turn Timer`)
  (`self.Play BGM`))

(event `EggsSettings`
  (params (`Host Eggs` :type "Array of /Game/Blueprints/Character/Egg_BlackKnight Object Reference") (`Client Eggs` :type "Array of /Game/Blueprints/Character/Egg_BlackKnight Object Reference"))
  ;[1 1 1] 알의 색깔 및 태그 세팅
  (for _array_element `Host Eggs`
    (bind _egg (`/Game/Blueprints/Character/Egg_BlackKnight.Egg` _array_element))
    (`KismetArrayLibrary.Array_AddUnique` (`ActorComponent.ComponentTags` _egg) "Host")
    (`PrimitiveComponent.SetMaterial` _egg 0 "/Engine/EditorMeshes/ColorCalibrator/M_ClearCoatBlack.M_ClearCoatBlack"))
  (for _array_element_2 `Client Eggs`
    (bind _egg_2 (`/Game/Blueprints/Character/Egg_BlackKnight.Egg` _array_element_2))
    (`KismetArrayLibrary.Array_AddUnique` (`ActorComponent.ComponentTags` _egg_2) "Client")
    (`PrimitiveComponent.SetMaterial` _egg_2 0 "/Game/Source/Materials/M_Metallic_White.M_Metallic_White")
    (`PrimitiveComponent.SetMaterial` (`/Game/Blueprints/Character/Egg_BlackKnight.Aura` _array_element_2) 0 "/Game/InfinityBladeEffects/Effects/FX_Materials/Noise/M_HealthShrine_01_INST.M_HealthShrine_01_INST")
    (`PrimitiveComponent.SetMaterial` (`/Game/Blueprints/Character/Egg_BlackKnight.Aura2` _array_element_2) 0 "/Game/InfinityBladeEffects/Effects/FX_Materials/Noise/M_HealthShrine_01_INST.M_HealthShrine_01_INST")))

(event `CameraSet`
  (params (NewParam :type "Float (double-precision)"))
  (bind _returnvalue (`GameplayStatics.GetPlayerController` 0))
  ;[1 1 1] 초기 카메라 시점으로 되돌리는 커스텀 이벤트
  (if (`KismetSystemLibrary.IsServer`)
    (`PlayerController.SetViewTargetWithBlend` _returnvalue (`|GetArrayItem` (`self.Cameras`)) NewParam "VTBlend_Linear" 0.0 true)
    (else
      (`PlayerController.SetViewTargetWithBlend` _returnvalue (`|GetArrayItem` (`self.Cameras`) 1) NewParam "VTBlend_Linear" 0.0 true))))

(event `Skill_Use`
  (params (Egg :type "/Game/Blueprints/Character/Egg_BlackKnight Object Reference"))
  (`/Game/Blueprints/Character/Egg_BlackKnight.Egg_Skill` Egg Egg))

(fn `CanSelect`
  (returns (NewParam :type Boolean))
  (locals (SetClick :type Boolean))
  (set `local.SetClick` false)
  (if (`KismetSystemLibrary.IsServer`)
    (if (== (mod (`self.TurnNum`) 2) 1)
      (set `local.SetClick` true)
      (else
        (set `local.SetClick` false)))
    (elif (== (mod (`self.TurnNum`) 2) 0)
      (set `local.SetClick` true)
      (else
        (set `local.SetClick` false))))
  (return (`local.SetClick`)))

(fn `Check Units Survival`
  (bind _hosteggs (`self.HostEggs`))
  (bind _clienteggs (`self.ClientEggs`))
  (`|ExecutionSequence`
    (:`then_0`
      (for _array_element (`self.ClientEggs`)
        (if (<= (`/Game/Blueprints/Character/Egg_BlackKnight.Current Health` _array_element) 0.0)
          (`/Game/Blueprints/Character/Egg_BlackKnight.Set Unit Dead(B)` _array_element)))
      (if (and (`/Game/Blueprints/Character/Egg_BlackKnight.Is Dead` (`|GetArrayItem` _clienteggs)) (`/Game/Blueprints/Character/Egg_BlackKnight.Is Dead` (`|GetArrayItem` _clienteggs 1)) (`/Game/Blueprints/Character/Egg_BlackKnight.Is Dead` (`|GetArrayItem` _clienteggs 2)) (`/Game/Blueprints/Character/Egg_BlackKnight.Is Dead` (`|GetArrayItem` _clienteggs 3)) (`/Game/Blueprints/Character/Egg_BlackKnight.Is Dead` (`|GetArrayItem` _clienteggs 4)))
        (`self.Show Result` true)))
    (:`then_1`
      (for _array_element_2 (`self.HostEggs`)
        (if (<= (`/Game/Blueprints/Character/Egg_BlackKnight.Current Health` _array_element_2) 0.0)
          (`/Game/Blueprints/Character/Egg_BlackKnight.Set Unit Dead(B)` _array_element_2)))
      (if (and (`/Game/Blueprints/Character/Egg_BlackKnight.Is Dead` (`|GetArrayItem` _hosteggs)) (`/Game/Blueprints/Character/Egg_BlackKnight.Is Dead` (`|GetArrayItem` _hosteggs 1)) (`/Game/Blueprints/Character/Egg_BlackKnight.Is Dead` (`|GetArrayItem` _hosteggs 2)) (`/Game/Blueprints/Character/Egg_BlackKnight.Is Dead` (`|GetArrayItem` _hosteggs 3)) (`/Game/Blueprints/Character/Egg_BlackKnight.Is Dead` (`|GetArrayItem` _hosteggs 4)))
        (`self.Show Result` false)))))

(fn `UserConstructionScript`)