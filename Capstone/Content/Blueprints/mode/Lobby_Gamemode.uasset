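; Lobby game mode that manages a two-player lobby with egg-character deck building and server-travels to BattleLevel.
; On authority, PostLogin registers each controller and sets up its lobby through Lobby_Control.
; EveryoneUpdate rebuilds ConnectedPlayers and pushes it to all controllers; map changes, kicks and logout save-slot deletion are also handled.
; DeckBuilding maps character IDs to eggs, writing into player 0 or 1 by status.
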(event `self.K2_PostLogin`
  (params (NewPlayer :type "PlayerController Object Reference"))
  ;[1 1 1] 로그인 이후 이벤트를 발동하는 초기 구성 단계 - 플레이어 컨트롤러에서 로비를 구성
  (`/Engine/EditorBlueprintResources/ActorMacros.Switch Has Authority`
    (:`Authority`
      (`KismetArrayLibrary.Array_Add` (`self.AllPlayerController`) NewPlayer)
      (bind _asmy_game_instance (cast `/Game/Blueprints/mode/MyGameInstance` (`GameplayStatics.GetGameInstance`)))
      (set `self.Server Name` (`/Game/Blueprints/mode/MyGameInstance.ServerName` _asmy_game_instance))
      (bind _aslobby_control (cast `/Game/Blueprints/mode/Lobby_Control` NewPlayer))
      (`/Game/Blueprints/mode/Lobby_Control.InitialSetup` _aslobby_control)
      (`/Game/Blueprints/mode/Lobby_Control.SetUpLobbyMenu` _aslobby_control (`self.Server Name`))
      (`/Game/Blueprints/mode/Lobby_Control.UpdateLobbySettings` _aslobby_control (`self.GM Map Name`))
      (`self.EveryoneUpdate`))))

(event `EveryoneUpdate`
  (bind _allplayercontroller (`self.AllPlayerController`))
  ;[1 1 1] 호출 시 접속자들에게 로비 정보 업데이트
  (bind _output_get (set `self.CurrentPlayers` (`KismetArrayLibrary.Array_Length` (`self.AllPlayerController`))))
  (if (> _output_get 0)
    (`KismetArrayLibrary.Array_Clear` (`self.ConnectedPlayers`))
    (for _array_element _allplayercontroller
      (bind _aslobby_control (cast `/Game/Blueprints/mode/Lobby_Control` _array_element))
      (`KismetArrayLibrary.Array_Add` (`self.ConnectedPlayers`) (`/Game/Blueprints/mode/Lobby_Control.Player Settings` _aslobby_control))
      (`/Game/Blueprints/mode/Lobby_Control.UpdateNumberOfPlayers` _aslobby_control (`self.CurrentPlayers`) 2))
    (for _array_element_2 _allplayercontroller
      (bind _aslobby_control_2 (cast `/Game/Blueprints/mode/Lobby_Control` _array_element_2))
      (`/Game/Blueprints/mode/Lobby_Control.AddPlayerInfo` _aslobby_control_2 (`self.ConnectedPlayers`))
      (`self.AddtoKickList`))))

(event `CannotStartGame`
  ;[1 1 1] 호출 시 접속자들에게 로비 정보 업데이트
  ;;[1 1 1] 영상에서 캐릭터를 선택 안했을 시 준비 버튼 안눌리게 하는 기능임, 추후 수정 유무 결정
  (for _array_element (`self.ConnectedPlayers`) :!via `Break`
    _))

(event `LaunchTheGame`
  ;[1 1 1] 맵 id에 따라 맵을 실행(추후 맵 id를 따로 설정해서 스위치에 연결 )
  (`KismetSystemLibrary.ExecuteConsoleCommand` "servertravel /Game/Maps/BattleLevel" (`GameplayStatics.GetPlayerController` 0)))

(event `ServerUpdateGameSettings`
  (params (MapName :type Text))
  ;[1 1 1] 서버에서 변동사항이 생기면 각 클라이언트에게 로비 정보를 업데이트하라고 통보(추후 맵 이미지, 맵 id를 입력에 추가해서 변수로 승격할 것)
  (set `self.GM Map Name` MapName)
  (for _array_element (`self.AllPlayerController`)
    (bind _aslobby_control (cast `/Game/Blueprints/mode/Lobby_Control` _array_element))
    (`/Game/Blueprints/mode/Lobby_Control.UpdateLobbySettings` _aslobby_control (`self.GM Map Name`))))

(event `RespawnPlayer`
  (params (`Player Controller` :type "PlayerController Object Reference"))
  (`self.EveryoneUpdate`))

(event `AddtoKickList`)

(event `YouHaveBeenKicked`
  (params (PlayerID :type Integer))
  ;[1 1 1] 선택한 플레이어를 로비에서 추방
  (`/Game/Blueprints/mode/Lobby_Control.Kicked` (cast `/Game/Blueprints/mode/Lobby_Control` (`|GetArrayItem` (`self.AllPlayerController`) PlayerID) :!pure true)))

(event `self.K2_OnLogout`
  (params (ExitingController :type "Controller Object Reference"))
  (bind _connectedplayers (`self.ConnectedPlayers`))
  ;[1 1 1] 로그아웃 이벤트가 플레이어 컨트롤러와 접속 정보를 없앰
  (for (_array_element _array_index) (`self.AllPlayerController`)
    (if (== _array_element ExitingController)
      (break)))
  (`KismetArrayLibrary.Array_Remove` (`self.AllPlayerController`) _array_index)
  (`KismetArrayLibrary.Array_Remove` _connectedplayers _array_index)
  (if (`KismetTextLibrary.EqualEqual_TextText` (`.MyPlayerStatus_17_BBFD6A7E491223E4AC2FB5BA3AB1BC9B` (break `/Game/Blueprints/mode/PlayerInfo` (`|GetArrayItem` _connectedplayers _array_index))) (`self.Building Condition`))
    (`GameplayStatics.DeleteGameInSlot` "HostSettingsSave")
    (else
      (`GameplayStatics.DeleteGameInSlot` "ClientSettingsSave")))
  (`self.EveryoneUpdate`))

(event `Deck Building`
  (params (`Character Count` :type Integer) (`Chracter ID` :type Integer) (`User Status` :type Text) (`Egg Deck` :type "Array of Pawn Class Reference (by ref)"))
  (bind _connectedplayers (`self.ConnectedPlayers`))
  (bind _connectedplayers_2 (`self.ConnectedPlayers`))
  (bind _player_deck (`self.Player Deck`))
  (bind (_myplayername _myeggdeck _myplayerstatus) (break `/Game/Blueprints/mode/PlayerInfo` (`|GetArrayItem` _connectedplayers_2 1)))
  (bind (_myplayername_2 _myeggdeck_2 _myplayerstatus_2) (break `/Game/Blueprints/mode/PlayerInfo` (`|GetArrayItem` _connectedplayers_2)))
  ;[1 1 1] 덱 구성
  (if (`KismetTextLibrary.EqualEqual_TextText` `User Status` (`self.Building Condition`))
    (bind _output_get (set `self.Player Deck` `Egg Deck`))
    (switch `int` `Chracter ID`
      (:`0`
        (`KismetArrayLibrary.Array_Set` _output_get `Character Count` "/Game/Blueprints/Character/Egg_Archer.Egg_Archer_C"))
      (:`1`
        (`KismetArrayLibrary.Array_Set` _output_get `Character Count` "/Game/Blueprints/Character/Egg_BlackKnight.Egg_BlackKnight_C"))
      (:`2`
        (`KismetArrayLibrary.Array_Set` _output_get `Character Count` "/Game/Blueprints/Character/Egg_GiantWoman.Egg_GiantWoman_C"))
      (:`3`
        (`KismetArrayLibrary.Array_Set` _output_get `Character Count` "/Game/Blueprints/Character/Egg_CastleWarrior.Egg_CastleWarrior_C"))
      (:`4`
        (`KismetArrayLibrary.Array_Set` _output_get `Character Count` "/Game/Blueprints/Character/Egg_Wizard.Egg_Wizard_C")))
    (setmembers `/Game/Blueprints/mode/PlayerInfo` :`StructRef` (`|GetArrayItem` _connectedplayers) :`MyPlayerName` _myplayername_2 :`MyEggDeck` _player_deck :`MyPlayerStatus` _myplayerstatus_2)
    (else
      (bind _output_get_2 (set `self.Player Deck` `Egg Deck`))
      (switch `int` `Chracter ID`
        (:`0`
          (`KismetArrayLibrary.Array_Set` _output_get_2 `Character Count` "/Game/Blueprints/Character/Egg_Archer.Egg_Archer_C"))
        (:`1`
          (`KismetArrayLibrary.Array_Set` _output_get_2 `Character Count` "/Game/Blueprints/Character/Egg_BlackKnight.Egg_BlackKnight_C"))
        (:`2`
          (`KismetArrayLibrary.Array_Set` _output_get_2 `Character Count` "/Game/Blueprints/Character/Egg_GiantWoman.Egg_GiantWoman_C"))
        (:`3`
          (`KismetArrayLibrary.Array_Set` _output_get_2 `Character Count` "/Game/Blueprints/Character/Egg_CastleWarrior.Egg_CastleWarrior_C"))
        (:`4`
          (`KismetArrayLibrary.Array_Set` _output_get_2 `Character Count` "/Game/Blueprints/Character/Egg_Wizard.Egg_Wizard_C")))
      (setmembers `/Game/Blueprints/mode/PlayerInfo` :`StructRef` (`|GetArrayItem` _connectedplayers 1) :`MyPlayerName` _myplayername :`MyEggDeck` _player_deck :`MyPlayerStatus` _myplayerstatus))))

(fn `UserConstructionScript`)