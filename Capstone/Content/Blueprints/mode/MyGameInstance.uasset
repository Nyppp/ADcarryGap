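; Game instance that drives front-end menu flow and multiplayer session hosting, joining and teardown.
; A save check opens the main menu, or options on first run; menu widgets are cached, except the server browser, rebuilt on each show.
; Hosting and joining show a loading screen, and successful session creation opens Lobby as a listen server.
; Failures route to DisplayErrorMsg, but it and both error-to-string helpers are empty stubs.
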(event `SaveGameCheck`
  ;[1 1 1] 저장 파일 확인
  (bind _returnvalue (`GameplayStatics.DoesSaveGameExist` (`self.PlayerSettingsSave`)))
  (if _returnvalue
    (`self.ShowMain`)
    (set `self.Created Save File` true)
    (else
      (`self.ShowOptions`)
      (set `PlayerController.bShowMouseCursor` true (`GameplayStatics.GetPlayerController` 0)))))

(event `ShowMain`
  ;[1 1 1] 메인 메뉴 출력
  (`/Engine/EditorBlueprintResources/StandardMacros.IsValid` (`self.Back Ground`)
    (:`Is Valid`
      _)
    (:`Is Not Valid`
      (bind _returnvalue (`|CreateWidget` "/Game/Blueprints/widget/WB_BackGround_Image.WB_BackGround_Image_C"))
      (set `self.Back Ground` _returnvalue)))
  (`UserWidget.AddToViewport` (`self.Back Ground`) 0)
  (`/Engine/EditorBlueprintResources/StandardMacros.IsValid` (`self.MainMenu`)
    (:`Is Valid`
      _)
    (:`Is Not Valid`
      (bind _returnvalue_2 (`|CreateWidget` "/Game/Blueprints/widget/WB_MainMenu.WB_MainMenu_C" (`GameplayStatics.GetPlayerController` 0)))
      (set `self.MainMenu` _returnvalue_2)))
  (`UserWidget.AddToViewport` (`self.MainMenu`) 0))

(event `ShowLoading`
  ;[1 1 1] 로딩 화면
  (`/Engine/EditorBlueprintResources/StandardMacros.IsValid` (`self.LoadingMenu`)
    (:`Is Valid`
      _)
    (:`Is Not Valid`
      (bind _returnvalue (`|CreateWidget` "/Game/Blueprints/widget/MultiPlay/Menu/WB_LoadingMenu.WB_LoadingMenu_C" (`GameplayStatics.GetPlayerController` 0)))
      (set `self.LoadingMenu` _returnvalue)))
  (`UserWidget.AddToViewport` (`self.LoadingMenu`) 0))

(event `self.HandleNetworkError`
  (params (FailureType :type "ENetworkFailure Enum" :default "NetDriverAlreadyExists") (bIsServer :type Boolean))
  ;[1 1 1] 에러처리
  (if bIsServer
    _
    (else
      _))
  (`self.DisplayErrorMsg` (`self.NetErrorToString` FailureType)))

(event `self.HandleTravelError`
  (params (FailureType :type "ETravelFailure Enum" :default "NoLevel"))
  ;[1 1 1] 에러처리
  (`self.DisplayErrorMsg` (`self.TravelErrorToString` FailureType)))

(event `ShowHost`
  ;[1 1 1] 호스트 메뉴(방 만들기) 출력
  (`/Engine/EditorBlueprintResources/StandardMacros.IsValid` (`self.HostMenu`)
    (:`Is Valid`
      _)
    (:`Is Not Valid`
      (bind _returnvalue (`|CreateWidget` "/Game/Blueprints/widget/MultiPlay/Menu/WB_HostMenu.WB_HostMenu_C" (`GameplayStatics.GetPlayerController` 0)))
      (set `self.HostMenu` _returnvalue)))
  (`UserWidget.AddToViewport` (`self.HostMenu`) 0))

(event `launch Lobby`
  (params (`Server Name` :type Text) (`Enable Lan` :type Boolean) (NumberOfPlayers :type Integer))
  ;[1 1 1] 방 생성
  (set `self.ServerName` `Server Name`)
  (`self.ShowLoading`)
  (`CreateSessionCallbackProxy.CreateSession` (`GameplayStatics.GetPlayerController` 0) NumberOfPlayers `Enable Lan`
    (:`OnSuccess`
      (`GameplayStatics.OpenLevel` "Lobby" true "listen"))
    (:`OnFailure`
      (`self.DisplayErrorMsg` "세션 생성 실패, 다시 시도해주세요"))))

(event `DestroySessionCaller`
  (params (PlayerController :type "PlayerController Object Reference"))
  ;[1 1 1] 세션 삭제
  (`DestroySessionCallbackProxy.DestroySession` PlayerController))

(event `JoinServer`
  (params (Session :type "BlueprintSessionResult Structure"))
  (bind _returnvalue (`GameplayStatics.GetPlayerController` 0))
  ;[1 1 1] 방 참가
  (`self.ShowLoading`)
  (`JoinSessionCallbackProxy.JoinSession` _returnvalue Session
    (:`OnFailure`
      (`self.DisplayErrorMsg` (`KismetSystemLibrary.GetDisplayName` _returnvalue)))))

(event `ShowServer`
  ;[1 1 1] 서버 메뉴 보여줌 -> 보여줄 때 마다 새로 만들어야 함
  (bind _returnvalue (`|CreateWidget` "/Game/Blueprints/widget/MultiPlay/Menu/WB_ServerMenu.WB_ServerMenu_C" (`GameplayStatics.GetPlayerController` 0)))
  (`UserWidget.AddToViewport` _returnvalue 0))

(event `ShowOptions`
  ;[1 1 1] 옵션 메뉴를 보여줌
  (`/Engine/EditorBlueprintResources/StandardMacros.IsValid` (`self.OptionMenu`)
    (:`Is Valid`
      _)
    (:`Is Not Valid`
      (bind _returnvalue (`|CreateWidget` "/Game/Blueprints/widget/MultiPlay/Menu/WB_OptionMenu.WB_OptionMenu_C" (`GameplayStatics.GetPlayerController` 0)))
      (set `self.OptionMenu` _returnvalue)))
  (`UserWidget.AddToViewport` (`self.OptionMenu`) 0))

(fn `NetErrorToString`
  (params (FailureType :type "ENetworkFailure Enum" :default "NetDriverAlreadyExists"))
  (returns (OutString :type String))
  (return ""))

(fn `TravelErrorToString`
  (params (`Failure Type` :type "ETravelFailure Enum" :default "NoLevel"))
  (returns (OutString :type String))
  (return ""))