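; Player controller for the Alkkagi egg-flicking game, handling aiming, shooting, skills and camera.
; Local BeginPlay loads saved host and client decks and passes them to the game mode for spawning.
; Tick aims the selected egg at the cursor; release shoots through the GameState, then advances the turn and deselects after a delay.
; Gates suspend normal shots during skill mode, while Archer skill targets follow the cursor, clamped to a radius.
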(event `self.ReceiveBeginPlay`
  ;[1 1 1] 플레이어 정보를 불러와 서버상 플레이어 컨트롤러에 넘겨줌
  (if (`self.IsLocalController`)
    (`WidgetLayoutLibrary.RemoveAllWidgets`)
    (`self.Load Game`)
    (`self.PassEggInfoToServer` (`self.HostSettings`) (`self.ClientSettings`))
    (else
      (bind _asalkkagi_game_state_base (cast `/Game/Blueprints/mode/AlkkagiGameStateBase` (`GameplayStatics.GetGameState`)))
      (`/Game/Blueprints/mode/AlkkagiGameStateBase.CameraSet` _asalkkagi_game_state_base 1.0))))

(event `self.ReceiveEndPlay`
  (params (EndPlayReason :type "EEndPlayReason Enum" :default "Destroyed"))
  ;[1 1 1] 클라가 나가도 호스트는 게임을 계속 해서 추가함 -> 클라가 나가면 세션 파기 후 레벨이동
)

(event `PassEggInfoToServer`
  (params (PlayerSetting :type "/Game/Blueprints/mode/PlayerInfo Structure") (PlayerSetting2 :type "/Game/Blueprints/mode/PlayerInfo Structure"))
  ;[1 1 1] 알 스폰
  (set `self.HostSettings` PlayerSetting)
  (set `self.ClientSettings` PlayerSetting2)
  (bind _asalkkagi_gamemode (cast `/Game/Blueprints/mode/Alkkagi_Gamemode` (`GameplayStatics.GetGameMode`)))
  (`/Game/Blueprints/mode/Alkkagi_Gamemode.RespawnPlayer` _asalkkagi_gamemode self (`.MyEggDeck_7_510706974AEFDB56D4AB088130FC1A75` (break `/Game/Blueprints/mode/PlayerInfo` (`self.HostSettings`))) (`.MyEggDeck_7_510706974AEFDB56D4AB088130FC1A75` (break `/Game/Blueprints/mode/PlayerInfo` (`self.ClientSettings`)))))

(event `UnPossessed`
  (params (egg :type "/Game/Blueprints/Character/Egg_BlackKnight Object Reference"))
  ;[1 1 1] 알의 선택 해제에 관련된 이벤트(불 변수, 화살표, 셀렉티드 에그 해제)
  (set `/Game/Blueprints/Character/Egg_BlackKnight.possessed` false egg)
  (`SceneComponent.SetVisibility` (`/Game/Blueprints/Character/Egg_BlackKnight.Active` egg) false false)
  (`SceneComponent.SetVisibility` (`/Game/Blueprints/Character/Egg_BlackKnight.Arrow` egg) false false)
  (set `self.Selected Egg` null)
  (set `/Game/Blueprints/Character/Egg_BlackKnight.IsCrashed` false egg)
  (set `self.Is Selected` false)
  (set `self.Is Shooted` false)
  (set `/Game/Blueprints/Character/Egg_BlackKnight.Egg Clicked` false egg)
  (cast `/Game/Blueprints/Character/Egg_Archer` egg
    (:`then`
      (`self.Reset_archer`))
    (:`CastFailed`
      (bind _asegg_castle_warrior (cast `/Game/Blueprints/Character/Egg_CastleWarrior` egg))
      (`/Game/Blueprints/Character/Egg_CastleWarrior.Skill_Destroy` _asegg_castle_warrior))))

(event `InputAxis|Turn`
  (params (AxisValue :type "Float (single-precision)"))
  ;[1 1 1] 선택 된 알에 대한 화면 회전, 확대
  (if (`self.Is Selected`)
    (`SceneComponent.K2_AddWorldRotation` (`/Game/Blueprints/Character/Egg_BlackKnight.SpringArm` (`self.Selected Egg`)) (`KismetMathLibrary.MakeRotator` 0.0 0.0 AxisValue) false true)))

(event `self.ReceiveTick`
  (params (DeltaSeconds :type "Float (single-precision)"))
  (bind _selected_egg (`self.Selected Egg`))
  ;[1 1 1] 선택된 알이 있을 시 틱마다 선택된 알 회전 / 선택된 알이 있을 경우 틱마다 알의 속도를 계산해서 알의 상태 변경
  (`|ExecutionSequence`
    (:`then_0`
      (if (not (`self.Is Shooted`))
        (`/Engine/EditorBlueprintResources/StandardMacros.IsValid` _selected_egg
          (:`Is Valid`
            (if (`/Game/Blueprints/Character/Egg_BlackKnight.Egg Clicked` _selected_egg)
              (`self.NotifyServerEggRotate` _selected_egg (`/Game/Blueprints/Character/Egg_BlackKnight.Egg Pos` _selected_egg) (`.Location` (`GameplayStatics.BreakHitResult` (`self.GetHitResultUnderCursorByChannel` (`GameplayStatics.GetPlayerController` 0) "TraceTypeQuery1" true)))))))))
    (:`then_1`
      (`self.Notify Cursor Location`))))

(event `InputAxis|Zoom`
  (params (AxisValue :type "Float (single-precision)"))
  (bind _springarm (`/Game/Blueprints/Character/Egg_BlackKnight.SpringArm` (`self.Selected Egg`)))
  ;[1 1 1] 선택 된 알에 대한 화면 회전, 확대
  (if (`self.Is Selected`)
    (set `SpringArmComponent.TargetArmLength` (+ (* AxisValue 100.0) (`SpringArmComponent.TargetArmLength` _springarm)) _springarm)))

(event `NotifyServerEggRotate`
  (params (`Selected Egg` :type "/Game/Blueprints/Character/Egg_BlackKnight Object Reference") (`Egg Position` :type "Vector Structure") (`Mouse Position` :type "Vector Structure"))
  ;[1 1 1] 선택된 알이 있을 시 틱마다 선택된 알 회전 / 선택된 알이 있을 경우 틱마다 알의 속도를 계산해서 알의 상태 변경
  (`self.ServerCauseEggRotate` `Selected Egg` `Egg Position` `Mouse Position`))

(event `Arrow Rain Zoom`
  (params (`Arrow Rain` :type "/Game/Blueprints/Character/SkillEffect/Archer_Skill Object Reference") (`Player Controller` :type "PlayerController Object Reference"))
  (`|ExecutionSequence`
    (:`then_0`
      (`/Engine/EditorBlueprintResources/ActorMacros.Switch Has Authority`
        (:`Authority`
          (`SceneComponent.K2_SetRelativeRotation` (`/Game/Blueprints/Character/SkillEffect/Archer_Skill.SpringArm` `Arrow Rain`) (`KismetMathLibrary.MakeRotator` 0.0 -35.0 (.yaw (`/Game/Blueprints/Character/Egg_BlackKnight.Egg Rotation` (`self.Selected Egg`)))) false false))))
    (:`then_1`
      (`self.SetViewTargetWithBlend` `Player Controller` `Arrow Rain` 0.2 "VTBlend_EaseIn" 1.5 false))))

(event `HitZoom`
  (params (`Hited Egg` :type "/Game/Blueprints/Character/Egg_BlackKnight Object Reference"))
  ;[1 1 1] 알이 상대 알에 히트시 카메라 타겟을 알로 옮김
  (`self.SetViewTargetWithBlend` self `Hited Egg` 1.0 "VTBlend_EaseIn" 1.0 false))

(event `ServerCauseEggRotate`
  (params (`Selected Egg` :type "/Game/Blueprints/Character/Egg_BlackKnight Object Reference") (`Egg Position` :type "Vector Structure") (`Mouse Position` :type "Vector Structure"))
  ;[1 1 1] 선택된 알이 있을 시 틱마다 선택된 알 회전 / 선택된 알이 있을 경우 틱마다 알의 속도를 계산해서 알의 상태 변경
  (`/Game/Blueprints/Character/Egg_BlackKnight.Rotate Arrow` `Selected Egg` `Egg Position` `Mouse Position`))

(event `InputAction|Shoot`
  (params (Key :type "Key Structure"))
  (bind _selected_egg (`self.Selected Egg`))
  ;[1 1 1] 일반 알 발사 / 아처 스킬을 구분짓기 위한 게이트
  (:`Pressed`
    (`|ExecutionSequence`
      (:`then_0`
        (`/Engine/EditorBlueprintResources/StandardMacros.Gate` false :!label _label
          (:`Exit`
            ;[1 1 1] 슛 입력
            (`/Engine/EditorBlueprintResources/StandardMacros.IsValid` _selected_egg
              (:`Is Valid`
                (`/Game/Blueprints/Character/Egg_BlackKnight.Egg Click` _selected_egg)
                (`KismetSystemLibrary.PrintString` "egg clicked"))))))
      (:`then_1`
        (`self.Execute Skill`))))
  (:`Released`
    (`/Engine/EditorBlueprintResources/StandardMacros.Gate` false :!label _label_2
      (:`Exit`
        (if (`/Game/Blueprints/Character/Egg_BlackKnight.Egg Clicked` (`self.Selected Egg`))
          (if (not (`self.Is Shooted`))
            (set `self.Is Shooted` true)
            (`SceneComponent.SetVisibility` (`/Game/Blueprints/Character/Egg_BlackKnight.Active` _selected_egg) false true)
            (`GameplayStatics.PlaySound2D` "/Engine/VREditor/Sounds/UI/Floating_UI_Close.Floating_UI_Close" 1.0 1.0 0.0 null null)
            (`self.NotifyServerShoot` (`self.Selected Egg`) (`.Location` (`GameplayStatics.BreakHitResult` (`self.GetHitResultUnderCursorByChannel` (`GameplayStatics.GetPlayerController` 0) "TraceTypeQuery1" true))))))))))

(event `Attacked Camera_Shake`
  ;[1 1 1] 충돌 시 카메라 흔들림, 효과
  (bind _returnvalue (`|CreateWidget` "/Game/Blueprints/widget/Blood_overlay.Blood_overlay_C" self))
  (`UserWidget.AddToViewport` _returnvalue 0)
  (`self.ClientStartCameraShake` "/Game/Blueprints/Crash_Camera.Crash_Camera_C" 1.5))

(event `Attack Camera Shake`
  ;[1 1 1] 충돌 시 카메라 흔들림, 효과
  (`self.ClientStartCameraShake` "/Game/Blueprints/Crash_Camera.Crash_Camera_C" 1.5))

(event `exit mouse skill mode`
  ;[1 1 1] 일반 알 발사 / 아처 스킬을 구분짓기 위한 게이트
  (`|ExecutionSequence`
    (:`then_0`
      (goto _label :!via `Open`))
    (:`then_1`
      (goto _label_2 :!via `Open`))))

(event `set mouse skill mode`
  ;[1 1 1] 일반 알 발사 / 아처 스킬을 구분짓기 위한 게이트
  (`|ExecutionSequence`
    (:`then_0`
      (goto _label :!via `Close`))
    (:`then_1`
      (goto _label_2 :!via `Close`))))

(event `Dead Camera Setting`
  (params (`Dead Egg` :type "/Game/Blueprints/Character/Egg_BlackKnight Object Reference"))
  ;[1 1 1] 알 사망 시 뷰 타깃 설정
  (if (== (`self.GetOwner` `Dead Egg`) self)
    (`self.SetViewTargetWithBlend` `Dead Egg` 0.5 "VTBlend_EaseIn")))

(event `NotifyServerShoot`
  (params (`Selected Egg` :type "/Game/Blueprints/Character/Egg_BlackKnight Object Reference") (`Mouse Pos` :type "Vector Structure"))
  ;[1 1 1] 슛 입력
  ;;[1 1 1] 슛 입력을 서버 동작으로 실행하기 위한 커스텀 이벤트
  (bind _asalkkagi_game_state_base (cast `/Game/Blueprints/mode/AlkkagiGameStateBase` (`GameplayStatics.GetGameState`)))
  (`/Game/Blueprints/mode/AlkkagiGameStateBase.State_Shoot` _asalkkagi_game_state_base `Selected Egg` `Mouse Pos`)
  (`KismetSystemLibrary.Delay` 4.0)
  (`/Game/Blueprints/mode/AlkkagiGameStateBase.AddTurn` _asalkkagi_game_state_base)
  (`self.UnPossessed` `Selected Egg`))

(event `Execute Skill`
  (bind _arrow_location (`self.Arrow_location`))
  ;[1 1 1] 아처 스킬 실행
  (`/Engine/EditorBlueprintResources/StandardMacros.DoOnce` false :!label _label_3
    (:`Completed`
      (bind _asegg_archer (cast `/Game/Blueprints/Character/Egg_Archer` (`self.Selected Egg`)))
      (bind _skill_actor (`/Game/Blueprints/Character/Egg_Archer.Skill Actor` _asegg_archer))
      (`self.K2_SetActorLocation` _skill_actor _arrow_location false false)
      (`/Game/Blueprints/Character/SkillEffect/Archer_Range.Execute Skill` _skill_actor _arrow_location))))

(event `Reset_archer`
  ;[1 1 1] 아처 스킬 실행
  (goto _label_3 :!via `Reset`))

(event `Notify Cursor Location`
  (bind _selected_egg (`self.Selected Egg`))
  (bind (_bblockinghit _binitialoverlap _time _distance _location) (`GameplayStatics.BreakHitResult` (`self.GetHitResultUnderCursorByChannel` "TraceTypeQuery1")))
  (bind _returnvalue (`SceneComponent.K2_GetComponentLocation` (`/Game/Blueprints/Character/Egg_BlackKnight.Egg` _selected_egg)))
  (bind _returnvalue_2 (- _location _returnvalue))
  (bind _returnvalue_3 (+ (* (/ (`KismetMathLibrary.MakeVector` (.x _returnvalue_2) (.y _returnvalue_2)) (`KismetMathLibrary.VSizeXY` _returnvalue_2)) 1000.0) _returnvalue))
  ;[1 1 1] 아처 스킬 사용 중 마우스 클릭 시, 해당 좌표 저장
  (bind _asegg_archer (cast `/Game/Blueprints/Character/Egg_Archer` _selected_egg))
  (if (< (`KismetMathLibrary.VSizeXY` (- _returnvalue _location)) 1000.0)
    (bind _skill_actor (`/Game/Blueprints/Character/Egg_Archer.Skill Actor` _asegg_archer))
    (`/Game/Blueprints/Character/SkillEffect/Archer_Range.Set Range Actor Location_Server` _skill_actor _location)
    (set `self.Arrow_location` _location)
    (else
      (`/Game/Blueprints/Character/SkillEffect/Archer_Range.Set Range Actor Location_Server` _skill_actor _returnvalue_3)
      (set `self.Arrow_location` _returnvalue_3))))

(fn `Load Game`
  (bind _returnvalue (`GameplayStatics.LoadGameFromSlot` (`self.HostSettingSave`)))
  (bind _asplayer_save_game (cast `/Game/Blueprints/mode/PlayerSaveGame` _returnvalue))
  (set `self.HostSettings` (`/Game/Blueprints/mode/PlayerSaveGame.S_PlayerInfo` _asplayer_save_game))
  (bind _returnvalue_2 (`GameplayStatics.LoadGameFromSlot` (`self.ClientSettingSave`)))
  (bind _asplayer_save_game_2 (cast `/Game/Blueprints/mode/PlayerSaveGame` _returnvalue_2))
  (set `self.ClientSettings` (`/Game/Blueprints/mode/PlayerSaveGame.S_PlayerInfo` _asplayer_save_game_2)))

(fn `UserConstructionScript`)