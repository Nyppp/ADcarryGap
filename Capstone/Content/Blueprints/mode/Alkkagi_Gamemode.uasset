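; Game mode for a two-player networked Alkkagi match that spawns each side's deck of eggs and cleans up when a player leaves.
; It caches Host and Client tagged TargetPoints and records controllers passed through OnSwapPlayerControllers.
; RespawnPlayer uses a counter to spawn host eggs first, then client eggs with a flipped camera arm, server-side as replicated actors owned by their controllers.
; Logout destroys the session through the GameInstance and deletes both settings saves.
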(event `self.ReceiveBeginPlay`
  ;[1 1 1] 초기 변수 셋업
  (bind _outactors (`GameplayStatics.GetAllActorsOfClassWithTag` "/Script/Engine.TargetPoint" "Host"))
  (set `self.Host Spawn` _outactors)
  (bind _outactors_2 (`GameplayStatics.GetAllActorsOfClassWithTag` "/Script/Engine.TargetPoint" "Client"))
  (set `self.Client Spawn` _outactors_2))

(event `self.K2_OnSwapPlayerControllers`
  (params (OldPC :type "PlayerController Object Reference") (NewPC :type "PlayerController Object Reference"))
  ;[1 1 1] 서버 접속자의 플레이어 컨트롤러 추적
  (`KismetArrayLibrary.Array_Add` (`self.AllPlayerControllers`) NewPC))

(event `RespawnPlayer`
  (params (PlayerController :type "PlayerController Object Reference") (`Host Deck` :type "Array of Pawn Class Reference") (`Client Deck` :type "Array of Pawn Class Reference"))
  ;[1 1 1] 초기 변수 셋업
  (if (== (`self.SpawnCondition`) 0)
    (for (_array_element _array_index) `Host Deck`
      (`/Engine/EditorBlueprintResources/ActorMacros.Switch Has Authority`
        (:`Authority`
          (bind _returnvalue (`|SpawnActorFromClass` _array_element (`self.GetTransform` (`|GetArrayItem` (`self.Host Spawn`) _array_index)) "AlwaysSpawn" "OverrideRootScale" (`|GetArrayItem` (`self.AllPlayerControllers`)) null))
          (bind _asegg_black_knight (cast `/Game/Blueprints/Character/Egg_BlackKnight` _returnvalue :!pure true))
          (`KismetArrayLibrary.Array_Add` (`self.Host Eggs`) _asegg_black_knight)
          (`self.SetReplicates` _asegg_black_knight true)
          (`self.SetReplicateMovement` _asegg_black_knight true)
          (set `/Game/Blueprints/Character/Egg_BlackKnight.Egg State` "NewEnumerator0" _asegg_black_knight))))
    (`/Engine/EditorBlueprintResources/StandardMacros.IncrementInt` (`self.SpawnCondition`))
    (else
      (for (_array_element_2 _array_index_2) `Client Deck`
        (`/Engine/EditorBlueprintResources/ActorMacros.Switch Has Authority`
          (:`Authority`
            (bind _returnvalue_2 (`|SpawnActorFromClass` _array_element_2 (`self.GetTransform` (`|GetArrayItem` (`self.Client Spawn`) _array_index_2)) "AlwaysSpawn" "OverrideRootScale" (`|GetArrayItem` (`self.AllPlayerControllers`) 1) null))
            (bind _asegg_black_knight_2 (cast `/Game/Blueprints/Character/Egg_BlackKnight` _returnvalue_2 :!pure true))
            (`KismetArrayLibrary.Array_Add` (`self.Client Eggs`) _asegg_black_knight_2)
            (`self.SetReplicates` _asegg_black_knight_2 true)
            (`self.SetReplicateMovement` _asegg_black_knight_2 true)
            (`SceneComponent.K2_SetRelativeRotation` (`/Game/Blueprints/Character/Egg_BlackKnight.SpringArm` _asegg_black_knight_2) (struct :`Pitch` -50.0 :`Yaw` 180.0) false false)
            (set `/Game/Blueprints/Character/Egg_BlackKnight.Egg State` "NewEnumerator2" _asegg_black_knight_2)))))))

(event `self.K2_OnLogout`
  (params (ExitingController :type "Controller Object Reference"))
  ;[1 1 1] 로그아웃 시 세션 파기
  (bind _asalkkagi_control (cast `/Game/Blueprints/mode/Alkkagi_Control` ExitingController))
  (`/Game/Blueprints/mode/MyGameInstance.DestroySessionCaller` (cast `/Game/Blueprints/mode/MyGameInstance` (`GameplayStatics.GetGameInstance`) :!pure true) _asalkkagi_control)
  (`GameplayStatics.DeleteGameInSlot` "HostSettingsSave")
  (`GameplayStatics.DeleteGameInSlot` "ClientSettingsSave"))

(fn `UserConstructionScript`)