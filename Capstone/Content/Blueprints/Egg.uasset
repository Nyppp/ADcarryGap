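; Egg is a turn-based piece that is launched by mouse aiming.
; Clicking it on its turn records the viewport mouse position and shows an arrow that Tick rotates and stretches toward the cursor.
; Shoot, not called within this graph, applies a velocity-change impulse along that screen-space offset, used directly as world XY.
; A two-second timer then unpossesses the player and ends the turn, which is exposed through getters and setters.
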(event `self.ReceiveTick`
  (params (DeltaSeconds :type "Float (single-precision)"))
  ;[1 1 1] 화살표
  (`self.Rotate Arrow` (stale `self.Egg.OnClicked` _output_get)))

(event `self.Egg.OnClicked`
  (params (TouchedComponent :type "PrimitiveComponent Object Reference") (ButtonPressed :type "Key Structure"))
  ;[1 1 1] 클릭 처리
  (bind _returnvalue (`self.Egg Click`))
  (bind _output_get (set `self.Egg_Pos` _returnvalue)))

(fn `Egg Click`
  (returns (ReturnValue :type "Vector2D Structure"))
  (if (`self.W_Turn`)
    (bind _output_get (set `self.Egg Clicked` true))
    (`SceneComponent.SetVisibility` (`self.Arrow`) _output_get false)
    (bind _returnvalue (`WidgetLayoutLibrary.GetMousePositionOnViewport`))
    (set `self.Egg_Pos` _returnvalue))
  (return _returnvalue))

(fn `Egg_UnPossess`
  (`Controller.UnPossess` (`GameplayStatics.GetPlayerController` 0))
  (set `self.W_Turn` false)
  (bind _output_get (set `self.Egg Clicked` false))
  (`SceneComponent.SetVisibility` (`self.Arrow`) _output_get false))

(fn `False_Turn`
  (set `self.W_Turn` false))

(fn `get_Clicked`
  (returns (Clicked :type Boolean))
  (return (`self.Egg Clicked`)))

(fn `get_Turn`
  (returns (Turn :type Boolean))
  (return (`self.W_Turn`)))

(fn `Rotate Arrow`
  (params (InVector2D :type "Vector2D Structure"))
  (bind _arrow (`self.Arrow`))
  (bind _returnvalue (`WidgetLayoutLibrary.GetMousePositionOnViewport`))
  (`SceneComponent.K2_SetWorldRotation` _arrow (`KismetMathLibrary.Conv_VectorToRotator` (- (`KismetMathLibrary.Conv_Vector2DToVector` _returnvalue) (`KismetMathLibrary.Conv_Vector2DToVector` InVector2D))) false false)
  (`SceneComponent.SetWorldScale3D` _arrow (`KismetMathLibrary.MakeVector` (/ (`KismetMathLibrary.Sqrt` (`KismetMathLibrary.DistanceSquared2D` _returnvalue InVector2D)) 45.0) 1.0 1.0)))

(fn `Shoot`
  (params (input :type "/Game/Blueprints/Egg Object Reference"))
  (if (`self.W_Turn`)
    (`SceneComponent.SetVisibility` (`/Game/Blueprints/Egg.Arrow` input) false true)
    (bind _returnvalue (`WidgetLayoutLibrary.GetMousePositionOnViewport`))
    (`PrimitiveComponent.AddImpulse` (`/Game/Blueprints/Egg.Egg` input) (* (- (`KismetMathLibrary.Conv_Vector2DToVector` (`self.Egg_Pos`)) (`KismetMathLibrary.Conv_Vector2DToVector` _returnvalue)) -8) "None" true)
    (`KismetSystemLibrary.K2_SetTimer` input "Egg_UnPossess" 2.0)))

(fn `True_Turn`
  (set `self.W_Turn` true))

(fn `UserConstructionScript`)